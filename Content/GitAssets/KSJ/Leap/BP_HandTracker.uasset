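; Leap hand tracker that turns received hand positions and gestures (Python coordinates) into light, angle and touch controls.
; GetClinetLocation range-maps finger positions to world and viewport coordinates, with a player-distance check for pointing.
; Right hand moves the light; left fist sends a time angle, and left point past the threshold sends a screen position, throttled to once per second.
; Left gestures fill a rolling history, but its majority vote is disconnected.
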(event `TouchReEnable`
  (goto _label :!via `Reset`))

(event `self.OnLeftHandDataReceived`
  (params (FingerPos :type "Vector Structure") (Gesture :type String) (Angle :type "Float (single-precision)"))
  (bind (_returnvalue _ispointingenablelocation _screenpositon) (`self.GetClinetLocation` FingerPos))
  (`|ExecutionSequence`
    (:`then_0`
      ; 왼손의 주먹, 보, 포인트중  가장 신뢰도 높은걸 실행
      (`|ExecutionSequence`
        (:`then_0`
          (switch `string` Gesture
            (:`FIST`
              (`KismetArrayLibrary.Array_Add` (`self.LeftRecords`)))
            (:`POINT`
              (`KismetArrayLibrary.Array_Add` (`self.LeftRecords`) 1))
            (:`OPEN`
              (`KismetArrayLibrary.Array_Add` (`self.LeftRecords`) 2))))
        (:`then_1`
          (if (`KismetStringLibrary.EqualEqual_StrStr` Gesture "FIST")
            ; 왼손 주먹 행동
            (`self.TimeAngle` Angle)))
        (:`then_2`
          (if (>= (`KismetArrayLibrary.Array_Length` (`self.LeftRecords`)) 10)
            (`KismetArrayLibrary.Array_Remove` (`self.LeftRecords`))))))
    (:`then_1`
      (if (`KismetStringLibrary.EqualEqual_StrStr` Gesture "POINT")
        (if _ispointingenablelocation
          (`/Engine/EditorBlueprintResources/StandardMacros.DoOnce` false :!label _label
            (:`Completed`
              (`self.GiveScreenPositionInfo` _screenpositon)
              (`KismetSystemLibrary.Delay` 1.0)
              (`self.TouchReEnable`))))))))

(event `OnHandDataReceived_1`
  (params (HandType :type String) (FingerPos :type "Vector Structure") (Gesture :type String) (Angle :type "Float (single-precision)"))
  ; 오른손은 제스쳐 상관없이
  (if (`KismetStringLibrary.EqualEqual_StrStr` HandType (`self.Right`))
    _))

(event `self.OnRightHandDataReceived`
  (params (FingerPos :type "Vector Structure") (Gesture :type String) (Angle :type "Float (single-precision)"))
  ; 손위치 전달
  (`self.UpdateLightLocation` (`self.GetClinetLocation` FingerPos)))

(fn `GetClinetLocation`
  (params (InVec :type "Vector Structure"))
  (returns (ReturnValue :type "Vector Structure") (IsPointingEnableLocation :type Boolean) (ScreenPositon :type "Vector2D Structure"))
  (locals (ScreenDistance :type "Float (double-precision)" :default 3000.0))
  (bind _x (.x InVec))
  (bind _z (.z InVec))
  (bind (_returnvalue_x _returnvalue_y) (`KismetMathLibrary.BreakVector2D` (`WidgetLayoutLibrary.GetViewportSize`)))
  (bind _returnvalue (`KismetMathLibrary.MakeVector` (`KismetMathLibrary.MapRangeClamped` (.y InVec) 0.7 0.2 20000.0 25000.0) (`KismetMathLibrary.MapRangeClamped` _x 0.17 0.5 1800.0 3800.0) (`KismetMathLibrary.MapRangeClamped` _z 0.7 0.38 -600.0 200.0)))
  (return _returnvalue (> (`KismetMathLibrary.Vector_Distance` (`self.K2_GetActorLocation` (`GameplayStatics.GetPlayerCharacter` 0)) _returnvalue) (`local.ScreenDistance`)) (/ (`KismetMathLibrary.MakeVector2D` (`KismetMathLibrary.MapRangeClamped` _x 0.17 0.96 0.0 _returnvalue_x) (`KismetMathLibrary.MapRangeClamped` _z 0.3 0.66 0.0 _returnvalue_y)) (`WidgetLayoutLibrary.GetViewportScale`))))

(fn `GetMostConfidentGesture`
  (returns (IsPoint :type Boolean))
  (locals (PointCount :type Integer) (OpenCount :type Integer) (FistCount :type Integer) (AllCount :type "Array of Integer"))
  (for _array_element (`self.LeftRecords`)
    (switch `int` _array_element
      (:`0`
        (`/Engine/EditorBlueprintResources/StandardMacros.IncrementInt` (`local.FistCount`)))
      (:`1`
        (`/Engine/EditorBlueprintResources/StandardMacros.IncrementInt` (`local.PointCount`)))
      (:`2`
        (`/Engine/EditorBlueprintResources/StandardMacros.IncrementInt` (`local.OpenCount`)))))
  ; 내림차순 정렬
  (`KismetArrayLibrary.Array_Add` (`local.AllCount`) (`local.FistCount`))
  (`KismetArrayLibrary.Array_Add` (`local.AllCount`) (`local.OpenCount`))
  (`KismetArrayLibrary.Array_Add` (`local.AllCount`) (`local.PointCount`))
  (`KismetArrayLibrary.SortIntArray` (`local.AllCount`) false "Descending")
  (for _array_element_2 (`local.AllCount`)
    ; Point가 최근에 제일 많음
    (if (== _array_element_2 (`local.PointCount`))
      (return true)
      (else
        ; FIST가 최근 제일 많음
        (if (== _array_element_2 (`local.FistCount`))
          (return false))))))

(fn `UserConstructionScript`)