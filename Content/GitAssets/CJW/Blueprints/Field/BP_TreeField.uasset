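; Field tree actor that grows, withers and changes between cherry blossom, maple, European and winter types, driven by external SetTree and UpdateTree calls.
; A randomly delayed recursive loop steps Level through per-type skinned meshes, pausing past mid-growth until a type change is requested.
; Level also drives falling-leaf Niagara spawn rate and maple color, with effects set only near the player.
; SwingTree adds a timeline rotation shake with a type-specific particle burst.
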(event `SwingTree`
  (bind (_firstrotation_roll _firstrotation_pitch _firstrotation_yaw) (`KismetMathLibrary.BreakRotator` (`self.FirstRotation`)))
  (set `self.FirstRotation` (`self.K2_GetActorRotation`))
  (bind (_direction _lerp) (`Timeline|SwingTimeline` :!via `PlayFromStart`)
    (:`Update`
      (`self.K2_SetActorRotation` (`KismetMathLibrary.RLerp` (`KismetMathLibrary.MakeRotator` (+ _firstrotation_roll (`KismetMathLibrary.RandomFloatInRange` -0.3)) (+ _firstrotation_pitch (`KismetMathLibrary.RandomFloatInRange` -0.3)) _firstrotation_yaw) (`KismetMathLibrary.MakeRotator` (+ _firstrotation_roll (`KismetMathLibrary.RandomFloatInRange` 0.0 0.3)) (+ _firstrotation_pitch (`KismetMathLibrary.RandomFloatInRange` 0.0 0.3)) _firstrotation_yaw) _lerp)))
    (:`Left`
      (`NiagaraFunctionLibrary.SpawnSystemAtLocation` (select `/Game/GitAssets/CJW/Enum/E_TreeType` (`self.TreeType`) :`NewEnumerator0` "/Game/GitAssets/CJW/VFX/Busrt/NS_BurstFallingBlossom.NS_BurstFallingBlossom" :`NewEnumerator1` "/Game/GitAssets/CJW/VFX/Falling/NS_FallingLeaves_Maple.NS_FallingLeaves_Maple" :`NewEnumerator2` "/Game/GitAssets/CJW/VFX/Falling/NS_FallingLeaves_GreenLeaf.NS_FallingLeaves_GreenLeaf" :`NewEnumerator3` "/Game/GitAssets/CJW/VFX/Busrt/NS_BurstFallingSnow.NS_BurstFallingSnow" :`NewEnumerator4` "/Game/GitAssets/CJW/VFX/Busrt/NS_BurstFallingBlossom.NS_BurstFallingBlossom" :!type "NiagaraSystem Object Reference") (+ (`SceneComponent.K2_GetComponentLocation` (`self.Niagara`)) (0.0 0.0 250.0)))
      (`self.K2_SetActorRotation` (`self.FirstRotation`)))))

(event `ChangeLeaf`
  ; 나무 각자 제어
  (`self.SetNiagara` true))

(event `SetTree`
  (params (InputType :type "/Game/GitAssets/CJW/Enum/E_TreeType Enum" :default "NewEnumerator0") (Level :type Integer))
  (bind _treetype (`self.TreeType`))
  ; 중앙 제어할때
  (set `self.TreeType` InputType)
  (set `self.Level` Level)
  (`KismetSystemLibrary.Delay` (`KismetMathLibrary.RandomFloatInRange` (* (`self.TimeRate`) 5.0) (* (`self.TimeRate`) 20.0)))
  (`self.SetSkeletonMesh` _treetype)
  (`self.SetFlowerColor` _treetype)
  (`self.SetNiagara` true))

(event `DieToFirstLevel`
  ; 나무 각자 제어
  (if (== (`self.Level`) 0)
    (if (`|EnumInequality` (`self.NextType`) (`self.TreeType`))
      ;; 새로운 시작
      (set `self.TreeType` (`self.NextType`))
      (`self.GrowToNextlevel`))
    (else
      (`/Engine/EditorBlueprintResources/StandardMacros.DecrementInt` (`self.Level`)
        (:`  `
          (`self.SetSkeletonMesh` (`self.TreeType`))
          (`KismetSystemLibrary.Delay` (`KismetMathLibrary.RandomFloatInRange` 0.0 (* (`self.TimeToGrow`) 0.5)))
          (`self.DieToFirstLevel`))))))

(event `ChangeToNextType`
  ; 나무 각자 제어
  ;; 형태 변환
  (set `self.Level` 0)
  (set `self.TreeType` (`self.NextType`))
  (set `self.WantChange` false)
  (`self.SetSkeletonMesh` (`self.TreeType`))
  (`KismetSystemLibrary.Delay` (`KismetMathLibrary.RandomFloatInRange` 0.0 (* (`self.TimeToGrow`) 0.5)))
  (`self.GrowToNextlevel`))

(event `GrowToNextlevel`
  ; 나무 각자 제어
  (bind _result (`/Engine/EditorBlueprintResources/StandardMacros.IncrementInt` (`self.Level`))
    (:`  `
      (`KismetSystemLibrary.Delay` (`KismetMathLibrary.RandomFloatInRange` 0.0 (`self.TimeToGrow`)))
      (if (>= _result 18)
        (`self.ChangeToNextType`)
        (else
          ;; 9렙 전까진 최고 상승
          (if (<= (`self.Level`) 9)
            (`self.SetSkeletonMesh` (`self.TreeType`) :!label _label)
            (`|ExecutionSequence`
              (:`then_0`
                ;; 일정량 나뭇잎이 있으면 나뭇잎 ㄹ어지게
                (if (and (>= (`self.Level`) 4) (<= (`self.Level`) 13))
                  (`self.ChangeLeaf`)
                  (else
                    (`self.SetNiagara` false))))
              (:`then_1`
                (`self.GrowToNextlevel`)))
            (else
              ;; 그 이상부턴 변화 원시
              (if (`self.WantChange`)
                (goto _label)))))))))

(event `self.ReceiveBeginPlay`)

(event `UpdateTree`
  (params (Type :type "/Game/GitAssets/CJW/Enum/E_TreeType Enum" :default "NewEnumerator0"))
  ; 나무 각자 제어
  (if (`|EnumInequality` Type (`self.TreeType`))
    (set `self.NextType` Type)
    ;; 레벨이 너무 낮으면 바로 변환
    (if (<= (`self.Level`) 5)
      (`self.ChangeToNextType`))
    (`self.SetGrowTermAccordingToType`)
    (set `self.WantChange` true)
    (set `self.TimeToGrow` (+ (`self.TimeToGrow`) -20.0))
    (else
      (set `self.TimeToGrow` (+ (`self.TimeToGrow`) 10.0)))))

(event `self.ReceiveTick`
  (params (DeltaSeconds :type "Float (single-precision)")))

(event `SetGrowTermAccordingToType`
  ; 나무마다 Term다르게
  (set `self.TimeToGrow` (* (select `/Game/GitAssets/CJW/Enum/E_TreeType` (`self.TreeType`) :`NewEnumerator0` 30.0 :`NewEnumerator1` 50.0 :`NewEnumerator2` 60.0 :`NewEnumerator3` 30.0 :`NewEnumerator4` 30.0) (`self.TimeRate`))))

(fn `SetFlowerColor`
  (params (TypeInput :type "/Game/GitAssets/CJW/Enum/E_TreeType Enum" :default "NewEnumerator0"))
  (switch `/Game/GitAssets/CJW/Enum/E_TreeType` TypeInput))

(fn `SetNiagara`
  (params (Active :type Boolean))
  (if Active
    (if (<= (`KismetMathLibrary.Vector_Distance` (`self.K2_GetActorLocation` (`GameplayStatics.GetPlayerCharacter` 0)) (`self.K2_GetActorLocation`)) 5000.0)
      (`NiagaraComponent.SetAsset` (`self.Niagara`) (select `/Game/GitAssets/CJW/Enum/E_TreeType` (`self.TreeType`) :`NewEnumerator0` "/Game/GitAssets/CJW/VFX/Falling/NS_CherryBlossomSystem.NS_CherryBlossomSystem" :`NewEnumerator1` "/Game/GitAssets/CJW/VFX/Falling/NS_FallingLeaves_Maple.NS_FallingLeaves_Maple" :`NewEnumerator2` "/Game/GitAssets/CJW/VFX/Falling/NS_FallingLeaves_GreenLeaf.NS_FallingLeaves_GreenLeaf" :!type "NiagaraSystem Object Reference") false)
      (`NiagaraComponent.SetVariableFloat` (`self.Niagara`) "SpawnRate" (select `int` (`self.Level`) :`0` 0.0 :`1` 0.0 :`2` 0.0 :`3` 5.0 :`4` 9.0 :`5` 11.0 :`6` 13.0 :`7` 15.0 :`8` 20.0 :`9` 25.0 :`10` 20.0 :`11` 15.0 :`12` 13.0 :`13` 11.0 :`14` 9.0 :`15` 5.0 :`16` 3.0 :`17` 1.0 :`18` 0.0 :!type "Float (single-precision)"))
      (switch `/Game/GitAssets/CJW/Enum/E_TreeType` (`self.TreeType`)
        (:`NewEnumerator1`
          (`NiagaraComponent.SetVariableLinearColor` (`self.Niagara`) "Color" (select `int` (`self.Level`) :`0` (struct :`R` 0.133 :`G` 0.545 :`B` 0.133 :`A` 1.0) :`1` (struct :`R` 0.196 :`G` 0.627 :`B` 0.196 :`A` 1.0) :`2` (struct :`R` 0.333 :`G` 0.667 :`B` 0.235 :`A` 1.0) :`3` (struct :`R` 0.471 :`G` 0.706 :`B` 0.196 :`A` 1.0) :`4` (struct :`R` 0.627 :`G` 0.745 :`B` 0.157 :`A` 1.0) :`5` (struct :`R` 0.784 :`G` 0.784 :`B` 0.118 :`A` 1.0) :`6` (struct :`R` 0.863 :`G` 0.627 :`B` 0.157 :`A` 1.0) :`7` (struct :`R` 0.863 :`G` 0.431 :`B` 0.118 :`A` 1.0) :`8` (struct :`R` 0.784 :`G` 0.314 :`B` 0.157 :`A` 1.0) :`9` (struct :`R` 0.745 :`G` 0.353 :`B` 0.196 :`A` 1.0) :`10` (struct :`R` 0.667 :`G` 0.392 :`B` 0.235 :`A` 1.0) :`11` (struct :`R` 0.864583 :`G` 0.392 :`B` 0.275 :`A` 1.0) :`12` (struct :`R` 0.549 :`G` 0.353 :`B` 0.235 :`A` 1.0) :`13` (struct :`R` 0.51 :`G` 0.314 :`B` 0.196 :`A` 1.0) :`14` (struct :`R` 0.431 :`G` 0.275 :`B` 0.157 :`A` 1.0) :`15` (struct :`R` 1.0 :`G` 0.255 :`B` 0.137 :`A` 1.0) :`16` (struct :`R` 0.392 :`G` 0.235 :`B` 0.118 :`A` 1.0) :`17` (struct :`R` 0.275 :`G` 0.196 :`B` 0.098 :`A` 1.0) :`18` (struct :`R` 0.275 :`G` 0.196 :`B` 0.098 :`A` 1.0) :!type "LinearColor Structure"))))
      (else
        (`NiagaraComponent.SetAsset` (`self.Niagara`) null true)))
    (else
      (`NiagaraComponent.SetAsset` (`self.Niagara`) null true))))

(fn `SetSkeletonMesh`
  (params (Selection :type "/Game/GitAssets/CJW/Enum/E_TreeType Enum" :default "NewEnumerator0"))
  ; cherry
  (switch `/Game/GitAssets/CJW/Enum/E_TreeType` Selection
    (:`NewEnumerator0`
      (`SkinnedMeshComponent.SetSkinnedAssetAndUpdate` (`self.InstancedSkinnedMesh`) (select `int` (`self.Level`) :`0` "/Game/DriveAssets/ForShare/CJW/Tree/CherryBlossom/Type1/CherryTree1.CherryTree1" :`1` "/Game/DriveAssets/ForShare/CJW/Tree/CherryBlossom/Type1/CherryTree2.CherryTree2" :`2` "/Game/DriveAssets/ForShare/CJW/Tree/CherryBlossom/Type1/CherryTree3.CherryTree3" :`3` "/Game/DriveAssets/ForShare/CJW/Tree/CherryBlossom/Type1/CherryTree4.CherryTree4" :`4` "/Game/DriveAssets/ForShare/CJW/Tree/CherryBlossom/Type1/CherryTree5.CherryTree5" :`5` "/Game/DriveAssets/ForShare/CJW/Tree/CherryBlossom/Type1/CherryTree6.CherryTree6" :`6` "/Game/DriveAssets/ForShare/CJW/Tree/CherryBlossom/Type1/CherryTree7.CherryTree7" :`7` "/Game/DriveAssets/ForShare/CJW/Tree/CherryBlossom/Type1/CherryTree8.CherryTree8" :`8` "/Game/DriveAssets/ForShare/CJW/Tree/CherryBlossom/Type1/CherryTree9.CherryTree9" :`9` "/Game/DriveAssets/ForShare/CJW/Tree/CherryBlossom/Type1/CherryTree10.CherryTree10" :`10` "/Game/DriveAssets/ForShare/CJW/Tree/CherryBlossom/Type1/CherryTree9.CherryTree9" :`11` "/Game/DriveAssets/ForShare/CJW/Tree/CherryBlossom/Type1/CherryTree8.CherryTree8" :`12` "/Game/DriveAssets/ForShare/CJW/Tree/CherryBlossom/Type1/CherryTree7.CherryTree7" :`13` "/Game/DriveAssets/ForShare/CJW/Tree/CherryBlossom/Type1/CherryTree6.CherryTree6" :`14` "/Game/DriveAssets/ForShare/CJW/Tree/CherryBlossom/Type1/CherryTree5.CherryTree5" :`15` "/Game/DriveAssets/ForShare/CJW/Tree/CherryBlossom/Type1/CherryTree4.CherryTree4" :`16` "/Game/DriveAssets/ForShare/CJW/Tree/CherryBlossom/Type1/CherryTree17.CherryTree17" :`17` "/Game/DriveAssets/ForShare/CJW/Tree/CherryBlossom/Type1/CherryTree18.CherryTree18" :`18` "/Game/DriveAssets/ForShare/CJW/Tree/CherryBlossom/Type1/CherryTree19.CherryTree19" :!type "SkinnedAsset Object Reference") false))
    (:`NewEnumerator1`
      ; Maple
      (`SkinnedMeshComponent.SetSkinnedAssetAndUpdate` (`self.InstancedSkinnedMesh`) (select `int` (`self.Level`) :`0` "/Game/DriveAssets/ForShare/CJW/Tree/Maple/Type1/MapleTree2.MapleTree2" :`1` "/Game/DriveAssets/ForShare/CJW/Tree/Maple/Type1/MapleTree2.MapleTree2" :`2` "/Game/DriveAssets/ForShare/CJW/Tree/Maple/Type1/MapleTree3.MapleTree3" :`3` "/Game/DriveAssets/ForShare/CJW/Tree/Maple/Type1/MapleTree4.MapleTree4" :`4` "/Game/DriveAssets/ForShare/CJW/Tree/Maple/Type1/MapleTree5.MapleTree5" :`5` "/Game/DriveAssets/ForShare/CJW/Tree/Maple/Type1/MapleTree6.MapleTree6" :`6` "/Game/DriveAssets/ForShare/CJW/Tree/Maple/Type1/MapleTree7.MapleTree7" :`7` "/Game/DriveAssets/ForShare/CJW/Tree/Maple/Type1/MapleTree8.MapleTree8" :`8` "/Game/DriveAssets/ForShare/CJW/Tree/Maple/Type1/MapleTree9.MapleTree9" :`9` "/Game/DriveAssets/ForShare/CJW/Tree/Maple/Type1/MapleTree10.MapleTree10" :`10` "/Game/DriveAssets/ForShare/CJW/Tree/Maple/Type1/MapleTree9.MapleTree9" :`11` "/Game/DriveAssets/ForShare/CJW/Tree/Maple/Type1/MapleTree8.MapleTree8" :`12` "/Game/DriveAssets/ForShare/CJW/Tree/Maple/Type1/MapleTree7.MapleTree7" :`13` "/Game/DriveAssets/ForShare/CJW/Tree/Maple/Type1/MapleTree6.MapleTree6" :`14` "/Game/DriveAssets/ForShare/CJW/Tree/Maple/Type1/MapleTree5.MapleTree5" :`15` "/Game/DriveAssets/ForShare/CJW/Tree/Maple/Type1/MapleTree4.MapleTree4" :`16` "/Game/DriveAssets/ForShare/CJW/Tree/Maple/Type1/MapleTree3.MapleTree3" :`17` "/Game/DriveAssets/ForShare/CJW/Tree/Maple/Type1/MapleTree2.MapleTree2" :`18` "/Game/DriveAssets/ForShare/CJW/Tree/CherryBlossom/Type1/CherryTree1.CherryTree1" :!type "SkinnedAsset Object Reference") false))
    (:`NewEnumerator2`
      ; European
      (`SkinnedMeshComponent.SetSkinnedAssetAndUpdate` (`self.InstancedSkinnedMesh`) (select `int` (`self.Level`) :`0` "/Game/DriveAssets/ForShare/CJW/Tree/European2/Type1/European2.European2" :`1` "/Game/DriveAssets/ForShare/CJW/Tree/European2/European2-1.European2-1" :`2` "/Game/DriveAssets/ForShare/CJW/Tree/European2/Type1/European3.European3" :`3` "/Game/DriveAssets/ForShare/CJW/Tree/European2/Type1/European4.European4" :`4` "/Game/DriveAssets/ForShare/CJW/Tree/European2/Type1/European5.European5" :`5` "/Game/DriveAssets/ForShare/CJW/Tree/European2/Type1/European6.European6" :`6` "/Game/DriveAssets/ForShare/CJW/Tree/European2/Type1/European7.European7" :`7` "/Game/DriveAssets/ForShare/CJW/Tree/European2/Type1/European8.European8" :`8` "/Game/DriveAssets/ForShare/CJW/Tree/European2/Type1/European9.European9" :`9` "/Game/DriveAssets/ForShare/CJW/Tree/European2/Type1/European10.European10" :`10` "/Game/DriveAssets/ForShare/CJW/Tree/European2/Type1/European9.European9" :`11` "/Game/DriveAssets/ForShare/CJW/Tree/European2/Type1/European8.European8" :`12` "/Game/DriveAssets/ForShare/CJW/Tree/European2/Type1/European7.European7" :`13` "/Game/DriveAssets/ForShare/CJW/Tree/European2/Type1/European6.European6" :`14` "/Game/DriveAssets/ForShare/CJW/Tree/European2/Type1/European5.European5" :`15` "/Game/DriveAssets/ForShare/CJW/Tree/European2/Type1/European4.European4" :`16` "/Game/DriveAssets/ForShare/CJW/Tree/European2/Type1/European3.European3" :`17` "/Game/DriveAssets/ForShare/CJW/Tree/European2/European16.European16" :`18` "/Game/DriveAssets/ForShare/CJW/Tree/European2/European17.European17" :!type "SkinnedAsset Object Reference") false))
    (:`NewEnumerator3`
      (`SkinnedMeshComponent.SetSkinnedAssetAndUpdate` (`self.InstancedSkinnedMesh`) "/Game/DriveAssets/ForShare/CJW/Tree/CherryBlossom/Type1/CherryTree1.CherryTree1" false :!label _label))
    (:`NewEnumerator4`
      (goto _label))))

(fn `UserConstructionScript`
  (set `self.TreeIdx` (`KismetMathLibrary.RandomIntegerInRange` 0 4))
  (`self.SetSkeletonMesh` "NewEnumerator4"))