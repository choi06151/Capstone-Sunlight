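; BP_FlowerField is a flower actor that displays one of six species at a growth stage set by Level.
; SetFlower waits a random GrowthSpeed-scaled delay, then swaps the single HISM instance's mesh or dissolves it via timeline.
; Scale grows with distance from PlayerStart, and distant flowers are hidden.
; SwingTree adds random sway and vegetation particles at high levels; the cluster-scattering trace function is never run.
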(event `SwingTree`
  (bind (_first_rotation_roll _first_rotation_pitch _first_rotation_yaw) (`KismetMathLibrary.BreakRotator` (`self.First Rotation`)))
  (set `self.First Rotation` (`self.K2_GetActorRotation`))
  (bind (_direction _lerp) (`Timeline|Timeline` :!via `PlayFromStart`)
    (:`Update`
      (`self.K2_SetActorRotation` (`KismetMathLibrary.RLerp` (`KismetMathLibrary.MakeRotator` (+ _first_rotation_roll (`KismetMathLibrary.RandomFloatInRange` -10.0 -2.0)) (+ _first_rotation_pitch (`KismetMathLibrary.RandomFloatInRange` -10.0 -2.0)) _first_rotation_yaw) (`KismetMathLibrary.MakeRotator` (+ _first_rotation_roll (`KismetMathLibrary.RandomFloatInRange` 2.0 10.0)) (+ _first_rotation_pitch (`KismetMathLibrary.RandomFloatInRange` 2.0 10.0)) _first_rotation_yaw) _lerp)))
    (:`Left`
      (`self.K2_SetActorRotation` (`self.First Rotation`))
      (if (>= (`self.Level`) 9)
        (`GameplayStatics.SpawnEmitterAtLocation` "/Game/Realistic_Starter_VFX_Pack_Vol2/Particles/Hit/P_Vegetation.P_Vegetation" (`self.K2_GetActorLocation`) (struct) (0.25 0.25 0.25))))))

(event `SetFlower`
  (params (InputType :type "/Game/GitAssets/CJW/Enum/E_FlowerType Enum" :default "NewEnumerator0") (Level :type Integer))
  (bind _growthspeed (`self.GrowthSpeed`))
  (bind _growthspeed_2 (`self.GrowthSpeed`))
  (`self.StopDie`)
  (set `self.Type` InputType)
  (if (== (`self.Level`) 13)
    (`KismetSystemLibrary.Delay` (`KismetMathLibrary.RandomFloatInRange` (* _growthspeed_2 5.0) (* _growthspeed_2 50.0)))
    (`self.StartDie`)
    (else
      (set `self.Level` Level)
      (`KismetSystemLibrary.Delay` (`KismetMathLibrary.RandomFloatInRange` (* _growthspeed 10.0) (* _growthspeed 50.0)))
      (if (`|EnumEquality` (`self.Type`) "NewEnumerator3")
        (if (== (`self.Level`) 0)
          (`self.StartDie`))
        (else
          (`self.SetStaticMesh`))))))

(event `SetGrwothSpeed`
  (params (GrowthSpeed :type "Float (single-precision)"))
  (set `self.GrowthSpeed` GrowthSpeed))

(event `self.ReceiveBeginPlay`)

(event `StartDie`
  (bind (_direction _fade) (`Timeline|Timeline_2` :!via `PlayFromStart` :!label _label)
    (:`Update`
      (`MeshComponent.SetScalarParameterValueOnMaterials` (`self.HISM_Cur`) "Dissolve" _fade))))

(event `StopDie`
  (goto _label :!via `Stop`))

(fn `CheckPlayerDistance`
  (returns (distance :type "Float (double-precision)"))
  (bind _returnvalue (`KismetMathLibrary.Vector_Distance` (`self.K2_GetActorLocation`) (`self.K2_GetActorLocation` (`self.PlayerStart`))))
  (if (>= _returnvalue 3000.0)
    (`self.SetActorHiddenInGame` true)
    (else
      (return (`KismetMathLibrary.MapRangeClamped` _returnvalue 0.0 3000.0 0.4 2.0)))))

(fn `GetRandomTransforms`
  (locals (MakedTransforms :type "Array of Transform Structure") (Location_Cur :type "Vector Structure"))
  (bind (_location_cur_x _location_cur_y) (`KismetMathLibrary.BreakVector` (`local.Location_Cur`)))
  (bind _returnvalue (+ (`KismetMathLibrary.MakeVector` _location_cur_x _location_cur_y 10000.0) (* (`KismetMathLibrary.RandomUnitVector`) (`KismetMathLibrary.RandomFloatInRange` 10.0 (`self.clusterRadius`)))))
  (set `local.Location_Cur` (`self.K2_GetActorLocation`))
  (for _ (range (+ (`KismetMathLibrary.RandomIntegerInRange` 1 (`self.clusterCount`)) 1))
    (bind _outhit (`KismetSystemLibrary.LineTraceSingle` _returnvalue (+ _returnvalue (0.0 0.0 -100000.0)) "TraceTypeQuery1"))
    (bind (_bblockinghit _binitialoverlap _time _distance _location _impactpoint _normal) (`GameplayStatics.BreakHitResult` _outhit))
    (if _bblockinghit
      (`KismetArrayLibrary.Array_Add` (`local.MakedTransforms`) (`KismetMathLibrary.MakeTransform` _location (`KismetMathLibrary.MakeRotFromZ` _normal) (`self.Scale`)))))
  (set `self.CurrentTransforms` (`local.MakedTransforms`))
  (return))

(fn `SetStaticMesh`
  (`InstancedStaticMeshComponent.ClearInstances` (`self.HISM_Cur`))
  (`|ExecutionSequence`
    (:`then_0`
      (switch `/Game/GitAssets/CJW/Enum/E_FlowerType` (`self.Type`)
        (:`NewEnumerator0`
          (`StaticMeshComponent.SetStaticMesh` (`self.HISM_Cur`) (select `int` (`self.Level`) :`0` "/Game/DriveAssets/NFlowerPack_4/Meshes/Bougainv/Bougainv_1_SM.Bougainv_1_SM" :`1` "/Game/DriveAssets/NFlowerPack_4/Meshes/Bougainv/Bougainv_2_SM.Bougainv_2_SM" :`2` "/Game/DriveAssets/NFlowerPack_4/Meshes/Bougainv/Bougainv_3_SM.Bougainv_3_SM" :`3` "/Game/DriveAssets/NFlowerPack_4/Meshes/Bougainv/Bougainv_4_SM.Bougainv_4_SM" :`4` "/Game/DriveAssets/NFlowerPack_4/Meshes/Bougainv/Bougainv_5_SM.Bougainv_5_SM" :`5` "/Game/DriveAssets/NFlowerPack_4/Meshes/Bougainv/Bougainv_6_SM.Bougainv_6_SM" :`6` "/Game/DriveAssets/NFlowerPack_4/Meshes/Bougainv/Bougainv_7_SM.Bougainv_7_SM" :`7` "/Game/DriveAssets/NFlowerPack_4/Meshes/Bougainv/Bougainv_8_SM.Bougainv_8_SM" :`8` "/Game/DriveAssets/NFlowerPack_4/Meshes/Bougainv/Bougainv_9_SM.Bougainv_9_SM" :`9` "/Game/DriveAssets/NFlowerPack_4/Meshes/Bougainv/Bougainv_10_SM.Bougainv_10_SM" :`10` "/Game/DriveAssets/NFlowerPack_4/Meshes/Bougainv/Bougainv_11_SM.Bougainv_11_SM" :`11` "/Game/DriveAssets/NFlowerPack_4/Meshes/Bougainv/Bougainv_12_SM.Bougainv_12_SM" :`12` "/Game/DriveAssets/NFlowerPack_4/Meshes/Bougainv/Bougainv_13_SM.Bougainv_13_SM" :!type "StaticMesh Object Reference"))
          (set `self.Scale` (* (`self.CheckPlayerDistance`) (0.4 0.4 0.4))))
        (:`NewEnumerator1`
          (`StaticMeshComponent.SetStaticMesh` (`self.HISM_Cur`) (select `int` (`self.Level`) :`0` "/Game/DriveAssets/NFlowerPack_4/Meshes/Dianthus/Dianthus_1_SM.Dianthus_1_SM" :`1` "/Game/DriveAssets/NFlowerPack_4/Meshes/Dianthus/Dianthus_2_SM.Dianthus_2_SM" :`2` "/Game/DriveAssets/NFlowerPack_4/Meshes/Dianthus/Dianthus_3_SM.Dianthus_3_SM" :`3` "/Game/DriveAssets/NFlowerPack_4/Meshes/Dianthus/Dianthus_4_SM.Dianthus_4_SM" :`4` "/Game/DriveAssets/NFlowerPack_4/Meshes/Dianthus/Dianthus_5_SM.Dianthus_5_SM" :`5` "/Game/DriveAssets/NFlowerPack_4/Meshes/Dianthus/Dianthus_6_SM.Dianthus_6_SM" :`6` "/Game/DriveAssets/NFlowerPack_4/Meshes/Dianthus/Dianthus_7_SM.Dianthus_7_SM" :`7` "/Game/DriveAssets/NFlowerPack_4/Meshes/Dianthus/Dianthus_8_SM.Dianthus_8_SM" :`8` "/Game/DriveAssets/NFlowerPack_4/Meshes/Dianthus/Dianthus_9_SM.Dianthus_9_SM" :`9` "/Game/DriveAssets/NFlowerPack_4/Meshes/Dianthus/Dianthus_10_SM.Dianthus_10_SM" :`10` "/Game/DriveAssets/NFlowerPack_4/Meshes/Dianthus/Dianthus_11_SM.Dianthus_11_SM" :`11` "/Game/DriveAssets/NFlowerPack_4/Meshes/Dianthus/Dianthus_12_SM.Dianthus_12_SM" :`12` "/Game/DriveAssets/NFlowerPack_4/Meshes/Dianthus/Dianthus_13_SM.Dianthus_13_SM" :!type "StaticMesh Object Reference"))
          (set `self.Scale` (* (`self.CheckPlayerDistance`) (0.65 0.65 0.65))))
        (:`NewEnumerator2`
          (`StaticMeshComponent.SetStaticMesh` (`self.HISM_Cur`) (select `int` (`self.Level`) :`0` "/Game/DriveAssets/NFlowerPack_4/Meshes/MontuakDaisy/MontuakDaisy_1_SM.MontuakDaisy_1_SM" :`1` "/Game/DriveAssets/NFlowerPack_4/Meshes/MontuakDaisy/MontuakDaisy_2_SM.MontuakDaisy_2_SM" :`2` "/Game/DriveAssets/NFlowerPack_4/Meshes/MontuakDaisy/MontuakDaisy_3_SM.MontuakDaisy_3_SM" :`3` "/Game/DriveAssets/NFlowerPack_4/Meshes/MontuakDaisy/MontuakDaisy_4_SM.MontuakDaisy_4_SM" :`4` "/Game/DriveAssets/NFlowerPack_4/Meshes/MontuakDaisy/MontuakDaisy_5_SM.MontuakDaisy_5_SM" :`5` "/Game/DriveAssets/NFlowerPack_4/Meshes/MontuakDaisy/MontuakDaisy_6_SM.MontuakDaisy_6_SM" :`6` "/Game/DriveAssets/NFlowerPack_4/Meshes/MontuakDaisy/MontuakDaisy_7_SM.MontuakDaisy_7_SM" :`7` "/Game/DriveAssets/NFlowerPack_4/Meshes/MontuakDaisy/MontuakDaisy_8_SM.MontuakDaisy_8_SM" :`8` "/Game/DriveAssets/NFlowerPack_4/Meshes/MontuakDaisy/MontuakDaisy_9_SM.MontuakDaisy_9_SM" :`9` "/Game/DriveAssets/NFlowerPack_4/Meshes/MontuakDaisy/MontuakDaisy_10_SM.MontuakDaisy_10_SM" :`10` "/Game/DriveAssets/NFlowerPack_4/Meshes/MontuakDaisy/MontuakDaisy_11_SM.MontuakDaisy_11_SM" :`11` "/Game/DriveAssets/NFlowerPack_4/Meshes/MontuakDaisy/MontuakDaisy_12_SM.MontuakDaisy_12_SM" :`12` "/Game/DriveAssets/NFlowerPack_4/Meshes/MontuakDaisy/MontuakDaisy_13_SM.MontuakDaisy_13_SM" :!type "StaticMesh Object Reference"))
          (set `self.Scale` (* (`self.CheckPlayerDistance`) (0.5 0.5 0.5))))
        (:`NewEnumerator4`
          (`StaticMeshComponent.SetStaticMesh` (`self.HISM_Cur`) (select `int` (`self.Level`) :`0` "/Game/DriveAssets/NFlowerPack_3/Meshes/Portulaca/Portulaca_1_SM.Portulaca_1_SM" :`1` "/Game/DriveAssets/NFlowerPack_3/Meshes/Portulaca/Portulaca_2_SM.Portulaca_2_SM" :`2` "/Game/DriveAssets/NFlowerPack_3/Meshes/Portulaca/Portulaca_3_SM.Portulaca_3_SM" :`3` "/Game/DriveAssets/NFlowerPack_3/Meshes/Portulaca/Portulaca_4_SM.Portulaca_4_SM" :`4` "/Game/DriveAssets/NFlowerPack_3/Meshes/Portulaca/Portulaca_5_SM.Portulaca_5_SM" :`5` "/Game/DriveAssets/NFlowerPack_3/Meshes/Portulaca/Portulaca_6_SM.Portulaca_6_SM" :`6` "/Game/DriveAssets/NFlowerPack_3/Meshes/Portulaca/Portulaca_7_SM.Portulaca_7_SM" :`7` "/Game/DriveAssets/NFlowerPack_3/Meshes/Portulaca/Portulaca_8_SM.Portulaca_8_SM" :`8` "/Game/DriveAssets/NFlowerPack_3/Meshes/Portulaca/Portulaca_9_SM.Portulaca_9_SM" :`9` "/Game/DriveAssets/NFlowerPack_3/Meshes/Portulaca/Portulaca_10_SM.Portulaca_10_SM" :`10` "/Game/DriveAssets/NFlowerPack_3/Meshes/Portulaca/Portulaca_11_SM.Portulaca_11_SM" :`11` "/Game/DriveAssets/NFlowerPack_3/Meshes/Portulaca/Portulaca_12_SM.Portulaca_12_SM" :`12` "/Game/DriveAssets/NFlowerPack_3/Meshes/Portulaca/Portulaca_13_SM.Portulaca_13_SM" :!type "StaticMesh Object Reference"))
          (set `self.Scale` (* (`self.CheckPlayerDistance`) (0.5 0.5 0.5))))
        (:`NewEnumerator5`
          (`StaticMeshComponent.SetStaticMesh` (`self.HISM_Cur`) (select `int` (`self.Level`) :`0` "/Game/DriveAssets/NFlowerPack_3/Meshes/Pentas/Pentas_1_SM.Pentas_1_SM" :`1` "/Game/DriveAssets/NFlowerPack_3/Meshes/Pentas/Pentas_2_SM.Pentas_2_SM" :`2` "/Game/DriveAssets/NFlowerPack_3/Meshes/Pentas/Pentas_3_SM.Pentas_3_SM" :`3` "/Game/DriveAssets/NFlowerPack_3/Meshes/Pentas/Pentas_4_SM.Pentas_4_SM" :`4` "/Game/DriveAssets/NFlowerPack_3/Meshes/Pentas/Pentas_5_SM.Pentas_5_SM" :`5` "/Game/DriveAssets/NFlowerPack_3/Meshes/Pentas/Pentas_6_SM.Pentas_6_SM" :`6` "/Game/DriveAssets/NFlowerPack_3/Meshes/Pentas/Pentas_7_SM.Pentas_7_SM" :`7` "/Game/DriveAssets/NFlowerPack_3/Meshes/Pentas/Pentas_8_SM.Pentas_8_SM" :`8` "/Game/DriveAssets/NFlowerPack_3/Meshes/Pentas/Pentas_9_SM.Pentas_9_SM" :`9` "/Game/DriveAssets/NFlowerPack_3/Meshes/Pentas/Pentas_10_SM.Pentas_10_SM" :`10` "/Game/DriveAssets/NFlowerPack_3/Meshes/Pentas/Pentas_11_SM.Pentas_11_SM" :`11` "/Game/DriveAssets/NFlowerPack_3/Meshes/Pentas/Pentas_12_SM.Pentas_12_SM" :`12` "/Game/DriveAssets/NFlowerPack_3/Meshes/Pentas/Pentas_13_SM.Pentas_13_SM" :!type "StaticMesh Object Reference"))
          (set `self.Scale` (* (`self.CheckPlayerDistance`) (0.5 0.5 0.5))))
        (:`NewEnumerator6`
          (`StaticMeshComponent.SetStaticMesh` (`self.HISM_Cur`) (select `int` (`self.Level`) :`0` "/Game/DriveAssets/NFlowerPack_3/Meshes/Leadwort/Leadwort_1_SM.Leadwort_1_SM" :`1` "/Game/DriveAssets/NFlowerPack_3/Meshes/Leadwort/Leadwort_2_SM.Leadwort_2_SM" :`2` "/Game/DriveAssets/NFlowerPack_3/Meshes/Leadwort/Leadwort_3_SM.Leadwort_3_SM" :`3` "/Game/DriveAssets/NFlowerPack_3/Meshes/Leadwort/Leadwort_4_SM.Leadwort_4_SM" :`4` "/Game/DriveAssets/NFlowerPack_3/Meshes/Leadwort/Leadwort_5_SM.Leadwort_5_SM" :`5` "/Game/DriveAssets/NFlowerPack_3/Meshes/Leadwort/Leadwort_6_SM.Leadwort_6_SM" :`6` "/Game/DriveAssets/NFlowerPack_3/Meshes/Leadwort/Leadwort_7_SM.Leadwort_7_SM" :`7` "/Game/DriveAssets/NFlowerPack_3/Meshes/Leadwort/Leadwort_8_SM.Leadwort_8_SM" :`8` "/Game/DriveAssets/NFlowerPack_3/Meshes/Leadwort/Leadwort_9_SM.Leadwort_9_SM" :`9` "/Game/DriveAssets/NFlowerPack_3/Meshes/Leadwort/Leadwort_10_SM.Leadwort_10_SM" :`10` "/Game/DriveAssets/NFlowerPack_3/Meshes/Leadwort/Leadwort_11_SM.Leadwort_11_SM" :`11` "/Game/DriveAssets/NFlowerPack_3/Meshes/Leadwort/Leadwort_12_SM.Leadwort_12_SM" :`12` "/Game/DriveAssets/NFlowerPack_3/Meshes/Leadwort/Leadwort_13_SM.Leadwort_13_SM" :!type "StaticMesh Object Reference"))
          (set `self.Scale` (* (`self.CheckPlayerDistance`) (0.5 0.5 0.5))))))
    (:`then_1`
      (`InstancedStaticMeshComponent.AddInstance` (`self.HISM_Cur`) (`self.GetTransform`) true)
      (`self.SetActorScale3D` (`self.Scale`))
      (`MeshComponent.SetScalarParameterValueOnMaterials` (`self.HISM_Cur`) "Dissolve" 0.0))))

(fn `UserConstructionScript`
  (bind _returnvalue (`GameplayStatics.GetActorOfClass` "/Script/Engine.PlayerStart"))
  (set `self.PlayerStart` _returnvalue)
  (`self.SetStaticMesh`))