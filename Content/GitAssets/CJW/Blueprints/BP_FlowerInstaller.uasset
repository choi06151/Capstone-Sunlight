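; Spawner actor that keeps placing BP_FlowerField actors at random spots around itself, each with a random flower type.
; From BeginPlay, SpawnFlower calls itself after every Installterm delay, spawning at a fixed high Z when ConfirmInstallPlace allows.
; ConfirmInstallPlace checks random XY points within SpawnRadius against the SpawnedLocation map.
; Its random offsets are separate pure calls, so checked, stored and returned points can differ.
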(event `self.ReceiveBeginPlay`
  (`self.SpawnFlower`))

(event `SpawnFlower`
  (bind (_notusing_ _loca) (`self.ConfirmInstallPlace`))
  (if (not _notusing_)
    (`|SpawnActorFromClass` "/Game/GitAssets/CJW/Blueprints/BP_FlowerField.BP_FlowerField_C" (`KismetMathLibrary.MakeTransform` (`KismetMathLibrary.MakeVector` (`KismetMathLibrary.BreakVector2D` _loca) (`.Y` (`KismetMathLibrary.BreakVector2D` _loca)) 10000.0)) "AlwaysSpawn" "MultiplyWithRoot" null 0 (cast `/Game/GitAssets/CJW/Enum/FlowerType` (`KismetMathLibrary.Conv_IntToByte` (`KismetMathLibrary.RandomIntegerInRange` 0 2))) 0.5 null))
  (`KismetSystemLibrary.Delay` (`self.Installterm`))
  (`self.SpawnFlower`))

(fn `ConfirmInstallPlace`
  (returns (`NotUsing?` :type Boolean) (Loca :type "Vector2D Structure"))
  (bind _spawnedlocation (`self.SpawnedLocation`))
  (bind _spawnradius (`self.SpawnRadius`))
  (bind _returnvalue (* _spawnradius -1.0))
  (bind (_returnvalue_x _returnvalue_y) (`KismetMathLibrary.BreakVector` (+ (`self.K2_GetActorLocation`) (`KismetMathLibrary.MakeVector` (`KismetMathLibrary.RandomFloatInRange` _returnvalue _spawnradius) (`KismetMathLibrary.RandomFloatInRange` _returnvalue _spawnradius) (`KismetMathLibrary.RandomFloatInRange` _returnvalue _spawnradius)))))
  (bind _returnvalue_2 (`KismetMathLibrary.MakeVector2D` _returnvalue_x _returnvalue_y))
  (if (`.ReturnValue` (`BlueprintMapLibrary.Map_Find` _spawnedlocation (`KismetMathLibrary.MakeVector2D` _returnvalue_x _returnvalue_y)))
    (return true (0.0 0.0))
    (else
      (`BlueprintMapLibrary.Map_Add` _spawnedlocation _returnvalue_2 true)
      (return false _returnvalue_2))))

(fn `UserConstructionScript`)