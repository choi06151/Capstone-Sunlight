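; A crow flock actor that repeatedly flies across a MiddlePoint at a set height, showing a random number of child birds per pass.
; A timeline moves it toward a randomized target derived from the previous angle, using cosine for both X and Y.
; After each pass it hides the birds, waits a random delay, restores their formation and flies again.
; GetForce, not called here, scatters the birds in alternating directions.
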(event `Initialized`
  (for _array_element (`SceneComponent.GetChildrenComponents` (`self.ParentBird`) false)
    (`SceneComponent.SetVisibility` _array_element false false)))

(event `self.ReceiveBeginPlay`
  (`self.StartMove`))

(event `SetCrowCount`
  (bind _output_get (set `self.CrowCount` (`KismetMathLibrary.RandomIntegerInRange` 0 (- (`SceneComponent.GetNumChildrenComponents` (`self.ParentBird`)) 1))))
  (for _index (range (+ _output_get 1))
    (`SceneComponent.SetVisibility` (`SceneComponent.GetChildComponent` (`self.ParentBird`) _index) true false)))

(event `StartMove`
  (set `self.PrevAngle` (`KismetMathLibrary.RandomFloatInRange` 0.0 360.0))
  (`self.MoveOtherSide`))

(event `MoveOtherSide`
  (bind _targetlocation (`self.TargetLocation`))
  (bind _startlocation (`self.StartLocation`))
  (bind (_returnvalue_x _returnvalue_y) (`KismetMathLibrary.BreakVector` (`self.K2_GetActorLocation` (`self.MiddlePoint`))))
  (bind _returnvalue (+ (+ (`self.PrevAngle`) 180.0) (`KismetMathLibrary.RandomFloatInRange` -30.0 30.0)))
  (bind _returnvalue_2 (`KismetMathLibrary.DegCos` _returnvalue))
  (`self.SetCrowCount`)
  (set `self.PrevAngle` _returnvalue)
  (set `self.StartLocation` (`self.K2_GetActorLocation`))
  (set `self.TargetLocation` (`KismetMathLibrary.MakeVector` (+ _returnvalue_x (* _returnvalue_2 (`self.DistanceToMain`))) (+ _returnvalue_y (* _returnvalue_2 (`self.DistanceToMain`))) (`self.CrowZHeight`)))
  (`TimelineComponent.SetPlayRate` (`self.MoveTimeline`) (`KismetMathLibrary.RandomFloatInRange` 0.6 0.8))
  (bind (_direction _newtrack_0) (`Timeline|MoveTimeline` :!via `PlayFromStart`)
    (:`Update`
      (`self.K2_SetActorLocation` (`KismetMathLibrary.VLerp` _startlocation _targetlocation _newtrack_0))
      (`self.K2_SetActorRotation` (`KismetMathLibrary.FindLookAtRotation` _startlocation _targetlocation)))
    (:`Finished`
      (`self.Initialized`)
      (`KismetSystemLibrary.Delay` (`KismetMathLibrary.RandomFloatInRange` 100.0 400.0))
      (`self.MakeOrigin`)
      (if (`KismetMathLibrary.RandomBool`)
        (`self.MoveOtherSide`)
        (else
          (`self.StartMove`))))))

(event `GetForce`
  (bind (_direction _newtrack_0) (`Timeline|Timeline` :!via `PlayFromStart`)
    (:`Update`
      (for (_array_element _array_index) (`SceneComponent.GetChildrenComponents` (`self.ParentBird`) false)
        (bind _returnvalue (* _newtrack_0 (`KismetMathLibrary.RandomFloatInRange` 12.0 24.0) (`KismetMathLibrary.SelectFloat` 1.0 -1.0 (== (mod _array_index 2) 0))))
        (`SceneComponent.K2_AddRelativeLocation` _array_element (`KismetMathLibrary.MakeVector` _returnvalue (* _returnvalue -1.0)) false false)))))

(event `MakeOrigin`
  (`SceneComponent.K2_SetRelativeLocation` (`self.Bird`) (90.0 -50.0 0.0) false false)
  (`SceneComponent.K2_SetRelativeLocation` (`self.Bird2`) (-160.0 -100.0 0.0) false false)
  (`SceneComponent.K2_SetRelativeLocation` (`self.Bird3`) (160.0 -100.0 0.0) false false)
  (`SceneComponent.K2_SetRelativeLocation` (`self.Bird4`) (220.0 -170.0 0.0) false false)
  (`SceneComponent.K2_SetRelativeLocation` (`self.Bird5`) (-240.0 -170.0 0.0) false false)
  (`SceneComponent.K2_SetRelativeLocation` (`self.Bird1`) (-90.0 -50.0 0.0) false false))

(fn `UserConstructionScript`)