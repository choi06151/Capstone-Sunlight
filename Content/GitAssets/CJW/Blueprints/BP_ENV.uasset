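; BP_ENV is the environment manager running the day/night cycle, seasons, clouds and weather.
; Looping timers advance the hour, animate sun rotation and color from curves, drift clouds and randomly swap the rain effect.
; Each day rollover advances season progress, updating post-processing, leaf creators, and foliage color and growth through timeline-blended Material Parameter Collections.
; DevelopTool overrides season, time, game speed and weather levels, driving Niagara rain/snow, wind and fog.
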(event `LerpValue`
  (set `self.TimeDetail` (`KismetMathLibrary.Conv_IntToDouble` (`self.TimeOfDay`)))
  (`KismetSystemLibrary.K2_ClearAndInvalidateTimerHandle` (`self.LerpValuetimer`))
  (bind _returnvalue (`KismetSystemLibrary.K2_SetTimerDelegate` (delegate `ApplyValue`) (* (`self.DaySpeed`) 0.15) true))
  (set `self.LerpValuetimer` _returnvalue))

(event `ApplyValue`
  (`self.ControlDirectionalLight`)
  (`self.ControlSkyAtmosphere`)
  (set `self.TimeDetail` (+ (`self.TimeDetail`) 0.01)))

(event `RefFun`
  (bind _outactors (`GameplayStatics.GetAllActorsOfClass` "/Game/GitAssets/CJW/Blueprints/BP_LeafCreator.BP_LeafCreator_C"))
  (set `self.LeafCreatosRef` _outactors))

(event `StartTimer`
  (`self.StartDayTimer`)
  (`self.StartRanEventTimer`)
  (`self.StartCloudChangeTimer`))

(event `Initilize`
  (`self.ControlCloudValue`)
  (`self.SeasonCal`)
  (`self.RefFun`))

(event `StartCloudChangeTimer`
  (`KismetSystemLibrary.K2_SetTimer` null "ControlCloudValue" 10.0 true))

(event `StartDayTimer`
  (`KismetSystemLibrary.K2_SetTimer` null "TimeCal" (* (`self.DaySpeed`) 15.0) true))

(event `ChangeSeasonForDebug`
  (params (Input :type "/Game/GitAssets/CJW/ESeason Enum" :default "NewEnumerator0"))
  (set `self.SeasonProgress` (select `/Game/GitAssets/CJW/ESeason` Input :`NewEnumerator0` 0.2 :`NewEnumerator1` 0.4 :`NewEnumerator2` 0.6 :`NewEnumerator3` 0.9))
  (`self.SeasonCal`))

(event `self.ReceiveBeginPlay`
  (`self.Initilize`)
  (`self.StartTimer`))

(event `StartRanEventTimer`
  (`KismetSystemLibrary.K2_SetTimer` null "RanTimeCal" (* (`self.DaySpeed`) 40.0) true))

(event `ControlGlobalTime+-`
  (params (ISUP :type Boolean))
  (bind _globaltime (`self.GlobalTime`))
  (bind _output_get (set `self.GlobalTime` (+ _globaltime (select `bool` ISUP :`false` 0.1 :`true` -0.1))))
  (`GameplayStatics.SetGlobalTimeDilation` _output_get)
  (`KismetSystemLibrary.PrintString` (`KismetStringLibrary.Conv_DoubleToString` _globaltime)))

(event `ControlGlobalTimeSet`
  (params (GlobalTime :type "Float (double-precision)"))
  (bind _output_get (set `self.GlobalTime` GlobalTime))
  (`GameplayStatics.SetGlobalTimeDilation` _output_get)
  (`KismetSystemLibrary.PrintString` (`KismetStringLibrary.Conv_DoubleToString` _output_get)))

(event `ControlSkyLight`
  (bind _lightcomponent (`SkyLight.LightComponent` (`self.SkyLightRef`)))
  (`SkyLightComponent.RecaptureSky` _lightcomponent)
  (`SkyLightComponent.SetIntensity` _lightcomponent (`CurveFloat.GetFloatValue` (`self.C_IntensityCurve`) (`self.TimeDetail`))))

(event `ControlDirectionalLight`
  (`LightComponent.SetTemperature` (`Light.LightComponent` (`self.DirectionalLightRef`)) (`CurveFloat.GetFloatValue` (`self.C_TemperatureCurve`) (`self.TimeDetail`)))
  (`LightComponent.SetLightColor` (`Light.LightComponent` (`self.DirectionalLightRef`)) (`CurveLinearColor.GetLinearColorValue` (`self.C_ColorCurve`) (`self.TimeDetail`)) true)
  (`SceneComponent.K2_SetWorldRotation` (`Light.LightComponent` (`self.DirectionalLightRef`)) (`KismetMathLibrary.MakeRotator` 78.0 (`CurveFloat.GetFloatValue` (`self.C_LightPitch`) (`self.TimeDetail`)) -25.0) false false))

(event `ControlSkyAtmosphere`)

(event `ControlEnvColor`
  (bind (_direction _lerp) (`Timeline|ChangeColorTimeline` :!via `PlayFromStart`)
    (:`Update`
      (`KismetMaterialLibrary.SetVectorParameterValue` "/Game/GitAssets/CJW/MaterialParameter/MP_ENVParameter.MP_ENVParameter" "GrassColorStart" (`KismetMathLibrary.LinearColorLerp` (`self.P_GrassColorStart`) (`self.N_GrassColorStart`) _lerp))
      (`KismetMaterialLibrary.SetVectorParameterValue` "/Game/GitAssets/CJW/MaterialParameter/MP_ENVParameter.MP_ENVParameter" "GrassColorEnd" (`KismetMathLibrary.LinearColorLerp` (`self.N_GrassColorEnd`) (`self.N_GrassColorEnd`) _lerp))
      (`KismetMaterialLibrary.SetVectorParameterValue` "/Game/GitAssets/CJW/MaterialParameter/MP_ENVParameter.MP_ENVParameter" "TreeColorStart" (`KismetMathLibrary.LinearColorLerp` (`self.P_TreeColorStart`) (`self.N_TreeColorStart`) _lerp))
      (`KismetMaterialLibrary.SetVectorParameterValue` "/Game/GitAssets/CJW/MaterialParameter/MP_ENVParameter.MP_ENVParameter" "TreeColorEnd" (`KismetMathLibrary.LinearColorLerp` (`self.P_TreeColorEnd`) (`self.N_TreeColorEnd`) _lerp))
      (`KismetMaterialLibrary.SetVectorParameterValue` "/Game/GitAssets/CJW/MaterialParameter/MP_ENVParameter.MP_ENVParameter" "GroundColor" (`KismetMathLibrary.LinearColorLerp` (`self.P_GroundColor`) (`self.N_GroundColor`) _lerp)))))

(event `ControlCloud`
  (params (P_Size :type "Float (double-precision)") (P_Speed :type "Float (double-precision)") (P_Storm :type "Float (double-precision)"))
  (bind (_direction _atoz) (`Timeline|CloudLerp` :!via `PlayFromStart`)
    (:`Update`
      ; -0.5~1
      (`KismetMaterialLibrary.SetScalarParameterValue` "/Game/GitAssets/CJW/MaterialParameter/MP_ENVParameter.MP_ENVParameter" "CloudSize" (`KismetMathLibrary.Lerp` P_Size (`self.CloudSize`) _atoz))
      ; 0~1
      (`KismetMaterialLibrary.SetScalarParameterValue` "/Game/GitAssets/CJW/MaterialParameter/MP_ENVParameter.MP_ENVParameter" "CloudSpeed" (`KismetMathLibrary.Lerp` P_Speed (`self.CloudSpeed`) _atoz))
      ; -0.2~0.5
      (`KismetMaterialLibrary.SetScalarParameterValue` "/Game/GitAssets/CJW/MaterialParameter/MP_ENVParameter.MP_ENVParameter" "CloudStorm" (`KismetMathLibrary.Lerp` P_Storm (`self.CloudStorm`) _atoz)))))

(event `ControlGrowth`
  (params (P_Tree :type "Float (double-precision)") (P_Grass :type "Float (double-precision)"))
  (bind (_direction _atoz) (`Timeline|GrowthTimeLine` :!via `PlayFromStart`)
    (:`Update`
      (`KismetMaterialLibrary.SetScalarParameterValue` "/Game/GitAssets/CJW/MaterialParameter/MP_ENVParameter.MP_ENVParameter" "TreeGrowth" (`KismetMathLibrary.Lerp` P_Tree (`self.TreeGrowth`) _atoz))
      (`KismetMaterialLibrary.SetScalarParameterValue` "/Game/GitAssets/CJW/MaterialParameter/MP_ENVParameter.MP_ENVParameter" "GrassGrowth" (`KismetMathLibrary.Lerp` P_Grass (`self.GrassGrowth`) _atoz)))))

(event `ControlClear`
  ; Rain=1 Normal = 0
  (`KismetMaterialLibrary.SetScalarParameterValue` "/Game/GitAssets/CJW/MaterialParameter/MP_WeatherParameter.MP_WeatherParameter" "RainSize")
  ; Rain=0 Normal=1
  (`KismetMaterialLibrary.SetScalarParameterValue` "/Game/GitAssets/CJW/MaterialParameter/MP_WeatherParameter.MP_WeatherParameter" "Roughness" 1.0)
  ; Rain=0 Normal=5
  (`KismetMaterialLibrary.SetScalarParameterValue` "/Game/GitAssets/CJW/MaterialParameter/MP_WeatherParameter.MP_WeatherParameter" "RainSurface" 5.0)
  ; Snow=1 Normal=0
  (`KismetMaterialLibrary.SetScalarParameterValue` "/Game/GitAssets/CJW/MaterialParameter/MP_WeatherParameter.MP_WeatherParameter" "Snow" 1.0)
  ; Rain=1 Normal=0
  (`KismetMaterialLibrary.SetScalarParameterValue` "/Game/GitAssets/CJW/MaterialParameter/MP_WeatherParameter.MP_WeatherParameter" "PostSetting_Drop")
  ; Rain=1 Normal=0
  (`KismetMaterialLibrary.SetScalarParameterValue` "/Game/GitAssets/CJW/MaterialParameter/MP_WeatherParameter.MP_WeatherParameter" "PostSetting_Drip"))

(event `ControlRain`
  (params (Level :type Integer))
  (bind _returnvalue (`KismetMathLibrary.RandomFloatInRange` -800.0 -1500.0))
  (bind _returnvalue_2 (`KismetMathLibrary.RandomFloatInRange` -1200.0 1200.0))
  (bind _niagara (`self.Niagara`))
  ; 0 to 1
  (`KismetMaterialLibrary.SetScalarParameterValue` "/Game/GitAssets/CJW/MaterialParameter/MP_WeatherParameter.MP_WeatherParameter" "RainSize" (select `int` Level :`0` 0.0 :`1` 0.2 :`2` 0.4 :`3` 0.6 :`4` 0.8 :!type "Float (single-precision)"))
  ; 1 to 0
  (`KismetMaterialLibrary.SetScalarParameterValue` "/Game/GitAssets/CJW/MaterialParameter/MP_WeatherParameter.MP_WeatherParameter" "Roughness" (select `int` Level :`0` 0.8 :`1` 0.6 :`2` 0.4 :`3` 0.2 :`4` 0.0 :!type "Float (single-precision)"))
  ; 비 애셋 교체
  (`NiagaraComponent.SetAsset` _niagara "/Game/GitAssets/CJW/VFX/NS_RainSystem.NS_RainSystem" true)
  ; 비 강수량 교체
  (`NiagaraComponent.SetVariableFloat` _niagara "SpawnRate" (select `int` Level :`0` 500.0 :`1` 1500.0 :`2` 5000.0 :`3` 7000.0 :`4` 8000.0 :!type "Float (single-precision)"))
  ; 방향설정
  (`NiagaraComponent.SetVariableVec3` (`self.Niagara`) "SpawnVelocityMin" (`KismetMathLibrary.MakeVector` 0.0 _returnvalue_2 _returnvalue))
  (`NiagaraComponent.SetVariableVec3` (`self.Niagara`) "SpawnVelocityMax" (`KismetMathLibrary.MakeVector` 0.0 (+ _returnvalue_2 500.0) (+ _returnvalue 300.0)))
  (`KismetMaterialLibrary.SetScalarParameterValue` "/Game/GitAssets/CJW/MaterialParameter/MP_WeatherParameter.MP_WeatherParameter" "PostSetting_Drop" (select `int` Level :`0` 0.001 :`1` 0.001 :`2` 0.001 :`3` 0.001 :!type "Float (single-precision)"))
  (`KismetMaterialLibrary.SetScalarParameterValue` "/Game/GitAssets/CJW/MaterialParameter/MP_WeatherParameter.MP_WeatherParameter" "PostSetting_Drip" (select `int` Level :`0` 0.05 :`1` 0.2 :`2` 0.4 :`3` 0.6 :!type "Float (single-precision)"))
  ; 5 to 1
  (`KismetMaterialLibrary.SetScalarParameterValue` "/Game/GitAssets/CJW/MaterialParameter/MP_WeatherParameter.MP_WeatherParameter" "RainSurface" (select `int` Level :`0` 5.0 :`1` 4.0 :`2` 3.0 :`3` 1.0 :!type "Float (single-precision)")))

(event `ControlSnow`
  (params (Level :type Integer))
  (`NiagaraComponent.SetAsset` (`self.Niagara`) "/Game/GitAssets/CJW/VFX/NS_SnowSystem.NS_SnowSystem" true)
  (`NiagaraComponent.SetVariableFloat` (`self.Niagara`) "SpawnRate" (select `int` Level :`0` 50.0 :`1` 300.0 :`2` 500.0 :`3` 700.0 :!type "Float (single-precision)"))
  (`NiagaraComponent.SetVariableVec3` (`self.Niagara`) "SpawnVelocity" (`KismetMathLibrary.MakeVector` 0.0 (`KismetMathLibrary.RandomFloatInRange` -200.0 200.0) (`KismetMathLibrary.RandomFloatInRange` -50.0 -200.0)))
  ; snow =  0  일반 = 1
  (`KismetMaterialLibrary.SetScalarParameterValue` "/Game/GitAssets/CJW/MaterialParameter/MP_WeatherParameter.MP_WeatherParameter" "Snow" (select `int` Level :`0` 0.8 :`1` 0.6 :`2` 0.4 :`3` 0.0 :!type "Float (single-precision)")))

(event `ControlWind`
  (params (Level :type Integer))
  (`KismetMaterialLibrary.SetScalarParameterValue` "/Game/DriveAssets/Mediterranean_Coast/World_Settings/MPC_GlobalWind.MPC_GlobalWind" "WindSpeed" (select `int` Level :`0` 2.0 :`1` 4.0 :`2` 7.0 :`3` 10.0 :!type "Float (single-precision)"))
  (`KismetMaterialLibrary.SetScalarParameterValue` "/Game/DriveAssets/Mediterranean_Coast/World_Settings/MPC_GlobalWind.MPC_GlobalWind" "WindNoise" (select `int` Level :`0` 1.0 :`1` 2.0 :`2` 3.0 :`3` 4.0 :!type "Float (single-precision)"))
  (`KismetMaterialLibrary.SetScalarParameterValue` "/Game/DriveAssets/Mediterranean_Coast/World_Settings/MPC_GlobalWind.MPC_GlobalWind" "WindStrength" (select `int` Level :`0` 5.0 :`1` 40.0 :`2` 80.0 :`3` 100.0 :!type "Float (single-precision)"))
  (`KismetMaterialLibrary.SetScalarParameterValue` "/Game/DriveAssets/Mediterranean_Coast/World_Settings/MPC_GlobalWind.MPC_GlobalWind" "WindTiling" (`KismetMathLibrary.RandomFloatInRange` 1.0 100.0)))

(event `ControlFog`
  (params (Level :type Integer))
  (`ExponentialHeightFogComponent.SetFogDensity` (`ExponentialHeightFog.Component` (`self.FogRef`)) (select `int` Level :`0` 0.0 :`1` 4.0 :`2` 7.0 :`3` 10.0 :!type "Float (single-precision)")))

(event `SeasonSet`
  (params (Input :type "Float (double-precision)"))
  ; SeasonSet
  (bind _output_get (set `self.SeasonProgress` Input))
  (`|ExecutionSequence`
    (:`then_0`
      (if (>= _output_get 1.1)
        (set `self.SeasonProgress` 0.0)))
    (:`then_1`
      (`self.SwitchSeason`)
      (`self.SetSeasonColor`)
      (`self.SetSeasonPostProcessSetting`)
      (`self.SetSeasonGrowth`))))

(event `TimeSet`
  (params (Input :type "Float (double-precision)"))
  ; TimeSet
  (set `self.TimeOfDay` (`KismetMathLibrary.FFloor` Input))
  (`|ExecutionSequence`
    (:`then_0`
      (if (>= (`self.TimeOfDay`) 25)
        (set `self.TimeOfDay` 1)
        (`self.SeasonCal`)))
    (:`then_1`
      (`self.UpdateTime`))
    (:`then_2`
      (`self.CalDayLight`))
    (:`then_3`
      (if (or (== (`self.TimeOfDay`) 5) (== (`self.TimeOfDay`) 7) (== (`self.TimeOfDay`) 21) (== (`self.TimeOfDay`) 18))
        (`self.SwitchTimePhase`)))))

(fn `ApplyTimePhase`
  (`|ExecutionSequence`
    (:`then_0`
      (switch `/Game/GitAssets/CJW/ETimePhase` (`self.CurrentTimePhase`)))))

(fn `CalDayLight`
  (`self.LerpValue`))

(fn `ControlCloudValue`
  (locals (P_Size :type "Float (double-precision)") (P_Speed :type "Float (double-precision)") (P_Storm :type "Float (double-precision)"))
  (bind _cloudsize (`self.CloudSize`))
  (bind _cloudspeed (`self.CloudSpeed`))
  (bind _cloudstorm (`self.CloudStorm`))
  (set `local.P_Size` _cloudsize)
  (set `self.CloudSize` (`KismetMathLibrary.FClamp` (+ _cloudsize (`KismetMathLibrary.RandomFloatInRange` -0.1 0.1)) -0.5))
  (set `local.P_Speed` _cloudspeed)
  (set `self.CloudSpeed` (`KismetMathLibrary.FClamp` (+ _cloudspeed (`KismetMathLibrary.RandomFloatInRange` -0.1 0.1))))
  (set `local.P_Storm` _cloudstorm)
  (set `self.CloudStorm` (`KismetMathLibrary.FClamp` (+ _cloudstorm (`KismetMathLibrary.RandomFloatInRange` -0.1 0.1)) -0.2 0.5))
  (`self.ControlCloud` (`local.P_Size`) (`local.P_Speed`) (`local.P_Storm`)))

(fn `DevelopTool`
  (params (Type :type "/Game/GitAssets/CJW/EDeveloperTool Enum" :default "NewEnumerator0") (Value :type "Float (double-precision)"))
  (`|ExecutionSequence`
    (:`then_0`
      (switch `/Game/GitAssets/CJW/EDeveloperTool` Type
        (:`NewEnumerator0`
          (`self.SeasonSet` (`local.Value`)))
        (:`NewEnumerator1`
          (`self.TimeSet` (`local.Value`)))
        (:`NewEnumerator2`
          (switch `/Game/GitAssets/CJW/ESeason` (`self.CurrentSeason`)
            (:`NewEnumerator0`
              (`self.ControlRain` (`KismetMathLibrary.FTrunc` (`local.Value`)) :!label _label))
            (:`NewEnumerator1`
              (goto _label))
            (:`NewEnumerator2`
              (goto _label))
            (:`NewEnumerator3`
              (`self.ControlSnow` (`KismetMathLibrary.FTrunc` (`local.Value`))))))
        (:`NewEnumerator3`
          (`self.ControlWind` (`KismetMathLibrary.FTrunc` (`local.Value`))))
        (:`NewEnumerator4`
          (`self.ControlFog` (`KismetMathLibrary.FTrunc` (`local.Value`))))
        (:`NewEnumerator5`
          (`self.ControlGlobalTimeSet` (`local.Value`)))))
    (:`then_1`
      (`self.UpdateTime`))))

(fn `RanTimeCal`
  (`NiagaraComponent.SetAsset` (`self.Niagara`) (select `int` (`KismetMathLibrary.RandomIntegerInRange` 0 5) :`0` "/Game/GitAssets/CJW/VFX/NS_RainSystem.NS_RainSystem" :`1` null :`2` null :`3` null :`4` null :`5` null :!type "NiagaraSystem Object Reference") true))

(fn `SeasonCal`
  (bind _output_get (set `self.SeasonProgress` (+ (`self.SeasonProgress`) 0.1)))
  (`|ExecutionSequence`
    (:`then_0`
      (if (>= _output_get 1.1)
        (set `self.SeasonProgress` 0.0)))
    (:`then_1`
      (`self.SwitchSeason`)
      (`self.SetSeasonColor`)
      (`self.SetSeasonPostProcessSetting`)
      (`self.SetSeasonGrowth`))))

(fn `SetSeasonColor`
  (bind _returnvalue (`KismetMathLibrary.FFloor` (* (`self.SeasonProgress`) 10.0)))
  (set `self.P_GrassColorStart` (`self.N_GrassColorStart`))
  (set `self.P_GrassColorEnd` (`self.N_GrassColorEnd`))
  (set `self.P_TreeColorStart` (`self.N_TreeColorStart`))
  (set `self.P_TreeColorEnd` (`self.N_TreeColorEnd`))
  (set `self.P_GroundColor` (`self.N_GroundColor`))
  (set `self.N_GrassColorStart` (select `int` _returnvalue :`0` (struct :`R` 0.67 :`G` 0.69 :`B` 0.71 :`A` 1.0) :`1` (struct :`R` 0.55 :`G` 0.65 :`B` 0.37 :`A` 1.0) :`2` (struct :`R` 0.37 :`G` 0.65 :`B` 0.37 :`A` 1.0) :`3` (struct :`R` 0.27 :`G` 0.55 :`B` 0.24 :`A` 1.0) :`4` (struct :`R` 0.24 :`G` 0.53 :`B` 0.22 :`A` 1.0) :`5` (struct :`R` 0.43 :`G` 0.55 :`B` 0.25 :`A` 1.0) :`6` (struct :`R` 0.43 :`G` 0.55 :`B` 0.25 :`A` 1.0) :`7` (struct :`R` 0.59 :`G` 0.53 :`B` 0.24 :`A` 1.0) :`8` (struct :`R` 0.47 :`G` 0.43 :`B` 0.25 :`A` 1.0) :`9` (struct :`R` 0.67 :`G` 0.69 :`B` 0.71 :`A` 1.0) :!type "LinearColor Structure"))
  (set `self.N_GrassColorEnd` (select `int` _returnvalue :`0` (struct :`R` 0.481661 :`G` 0.496039 :`B` 0.510417 :`A` 1.0) :`1` (struct :`R` 0.489693 :`G` 0.65 :`B` 0.290571 :`A` 1.0) :`2` (struct :`R` 0.301977 :`G` 0.65 :`B` 0.343118 :`A` 1.0) :`3` (struct :`R` 0.177977 :`G` 0.55 :`B` 0.157981 :`A` 1.0) :`4` (struct :`R` 0.122339 :`G` 0.53 :`B` 0.11009 :`A` 1.0) :`5` (struct :`R` 0.413115 :`G` 0.55 :`B` 0.155352 :`A` 1.0) :`6` (struct :`R` 0.41595 :`G` 0.55 :`B` 0.161007 :`A` 1.0) :`7` (struct :`R` 0.59 :`G` 0.53 :`B` 0.24 :`A` 1.0) :`8` (struct :`R` 0.47 :`G` 0.430348 :`B` 0.406354 :`A` 1.0) :`9` (struct :`R` 0.771329 :`G` 0.78125 :`B` 0.729781 :`A` 1.0) :!type "LinearColor Structure"))
  (set `self.N_TreeColorStart` (select `int` _returnvalue :`0` (struct :`R` 0.47 :`G` 0.47 :`B` 0.47 :`A` 1.0) :`1` (struct :`R` 0.59 :`G` 0.63 :`B` 0.43 :`A` 1.0) :`2` (struct :`R` 1.0 :`G` 0.75 :`B` 0.8 :`A` 1.0) :`3` (struct :`R` 0.29 :`G` 0.59 :`B` 0.25 :`A` 1.0) :`4` (struct :`R` 0.044436 :`G` 0.249 :`B` 0.035539 :`A` 1.0) :`5` (struct :`R` 0.65 :`G` 0.390727 :`B` 0.210678 :`A` 1.0) :`6` (struct :`R` 0.76 :`G` 0.576887 :`B` 0.285 :`A` 1.0) :`7` (struct :`R` 0.76 :`G` 0.708786 :`B` 0.40516 :`A` 1.0) :`8` (struct :`R` 0.55 :`G` 0.487533 :`B` 0.331089 :`A` 1.0) :`9` (struct :`R` 0.47 :`G` 0.47 :`B` 0.47 :`A` 1.0) :!type "LinearColor Structure"))
  (set `self.N_TreeColorEnd` (select `int` _returnvalue :`0` (struct :`R` 0.6875 :`G` 0.6875 :`B` 0.6875 :`A` 1.0) :`1` (struct :`R` 0.554861 :`G` 0.63 :`B` 0.301875 :`A` 1.0) :`2` (struct :`R` 3.0 :`G` 2.25 :`B` 2.4 :`A` 1.0) :`3` (struct :`R` 0.20012 :`G` 0.59 :`B` 0.134627 :`A` 1.0) :`4` (struct :`R` 0.024107 :`G` 0.114583 :`B` 0.025561 :`A` 1.0) :`5` (struct :`R` 0.7 :`G` 0.121252 :`B` 0.086416 :`A` 1.0) :`6` (struct :`R` 0.76 :`G` 0.323674 :`B` 0.043771 :`A` 1.0) :`7` (struct :`R` 0.76 :`G` 0.672457 :`B` 0.474012 :`A` 1.0) :`8` (struct :`R` 0.55 :`G` 0.498157 :`B` 0.327151 :`A` 1.0) :`9` (struct :`R` 0.255208 :`G` 0.255208 :`B` 0.255208 :`A` 1.0) :!type "LinearColor Structure"))
  (set `self.N_GroundColor` (* (`self.N_GrassColorStart`) (struct :`R` 1.1 :`G` 1.05 :`B` 0.9 :`A` 1.0)))
  (`self.ControlEnvColor`))

(fn `SetSeasonGrowth`
  (locals (P_Tree :type "Float (double-precision)") (P_Grass :type "Float (double-precision)"))
  (set `local.P_Tree` (`self.TreeGrowth`))
  (set `local.P_Grass` (`self.GrassGrowth`))
  (set `self.TreeGrowth` (select `int` (`KismetMathLibrary.FFloor` (* (`self.SeasonProgress`) 10.0)) :`0` 0.0 :`1` 0.0 :`2` 1.0 :`3` 0.0 :`4` 1.0 :`5` 1.0 :`6` 1.0 :`7` 0.0 :`8` 0.0 :`9` 0.0))
  (set `self.GrassGrowth` (select `int` (`KismetMathLibrary.FFloor` (* (`self.SeasonProgress`) 10.0)) :`0` 0.1 :`1` 0.1 :`2` 0.1 :`3` 0.4 :`4` 0.5 :`5` 0.6 :`6` 1.0 :`7` 0.7 :`8` 0.4 :`9` 0.1))
  (`self.ControlGrowth` (`local.P_Tree`) (`local.P_Grass`)))

(fn `SetSeasonPostProcessSetting`
  (bind _postprocessref (`self.PostProcessRef`))
  (bind _returnvalue (`CurveFloat.GetFloatValue` (`self.C_PostContrast`) (* (`self.SeasonProgress`) 10.0)))
  (bind _returnvalue_2 (`CurveFloat.GetFloatValue` (`self.C_PostSaturation`) (* (`self.SeasonProgress`) 10.0)))
  (bind _structout (setmembers `PostProcessSettings` :`StructRef` (`PostProcessVolume.Settings` _postprocessref) :`WhiteTemp` (`CurveFloat.GetFloatValue` (`self.C_PostTemperature`) (* (`self.SeasonProgress`) 10.0)) :`WhiteTint` (`CurveFloat.GetFloatValue` (`self.C_PostTint`) (* (`self.SeasonProgress`) 10.0)) :`ColorSaturation` (`KismetMathLibrary.MakeVector4` _returnvalue_2 _returnvalue_2 _returnvalue_2 _returnvalue_2) :`ColorContrast` (`KismetMathLibrary.MakeVector4` _returnvalue _returnvalue _returnvalue _returnvalue)))
  (set `PostProcessVolume.Settings` _structout _postprocessref))

(fn `SwitchSeason`
  (set `self.CurrentSeason` (select `int` (`KismetMathLibrary.FFloor` (* (`self.SeasonProgress`) 10.0)) :`0` "NewEnumerator3" :`1` "NewEnumerator3" :`2` "NewEnumerator3" :`3` "NewEnumerator0" :`4` "NewEnumerator1" :`5` "NewEnumerator1" :`6` "NewEnumerator1" :`7` "NewEnumerator2" :`8` "NewEnumerator2" :`9` "NewEnumerator3" :!type "/Game/GitAssets/CJW/ESeason Enum"))
  ; 나무에서 떨어지는 꽃 변화
  (for _array_element (`self.LeafCreatosRef`)
    (`/Game/GitAssets/CJW/Blueprints/BP_LeafCreator.ChangeLeaf` _array_element (`self.SeasonProgress`))))

(fn `SwitchTimePhase`
  (switch `/Game/GitAssets/CJW/ESeason` (`self.CurrentSeason`)
    (:`NewEnumerator0`
      ; 봄
      (set `self.CurrentTimePhase` (select `int` (`self.TimeOfDay`) :`0` "NewEnumerator4" :`1` "NewEnumerator4" :`2` "NewEnumerator4" :`3` "NewEnumerator4" :`4` "NewEnumerator4" :`5` "NewEnumerator0" :`6` "NewEnumerator0" :`7` "NewEnumerator1" :`8` "NewEnumerator1" :`9` "NewEnumerator2" :`10` "NewEnumerator2" :`11` "NewEnumerator2" :`12` "NewEnumerator2" :`13` "NewEnumerator2" :`14` "NewEnumerator2" :`15` "NewEnumerator2" :`16` "NewEnumerator2" :`17` "NewEnumerator2" :`18` "NewEnumerator3" :`19` "NewEnumerator3" :`20` "NewEnumerator3" :`21` "NewEnumerator3" :`22` "NewEnumerator4" :`23` "NewEnumerator4" :`24` "NewEnumerator4" :!type "/Game/GitAssets/CJW/ETimePhase Enum")))
    (:`NewEnumerator1`
      ; 여름
      (set `self.CurrentTimePhase` (select `int` (`self.TimeOfDay`) :`0` "NewEnumerator4" :`1` "NewEnumerator4" :`2` "NewEnumerator4" :`3` "NewEnumerator4" :`4` "NewEnumerator0" :`5` "NewEnumerator0" :`6` "NewEnumerator1" :`7` "NewEnumerator1" :`8` "NewEnumerator1" :`9` "NewEnumerator2" :`10` "NewEnumerator2" :`11` "NewEnumerator2" :`12` "NewEnumerator2" :`13` "NewEnumerator2" :`14` "NewEnumerator2" :`15` "NewEnumerator2" :`16` "NewEnumerator2" :`17` "NewEnumerator2" :`18` "NewEnumerator2" :`19` "NewEnumerator3" :`20` "NewEnumerator3" :`21` "NewEnumerator3" :`22` "NewEnumerator4" :`23` "NewEnumerator4" :`24` "NewEnumerator4" :!type "/Game/GitAssets/CJW/ETimePhase Enum")))
    (:`NewEnumerator2`
      ; 가을
      (set `self.CurrentTimePhase` (select `int` (`self.TimeOfDay`) :`0` "NewEnumerator4" :`1` "NewEnumerator4" :`2` "NewEnumerator4" :`3` "NewEnumerator4" :`4` "NewEnumerator4" :`5` "NewEnumerator0" :`6` "NewEnumerator0" :`7` "NewEnumerator1" :`8` "NewEnumerator1" :`9` "NewEnumerator1" :`10` "NewEnumerator2" :`11` "NewEnumerator2" :`12` "NewEnumerator2" :`13` "NewEnumerator2" :`14` "NewEnumerator2" :`15` "NewEnumerator2" :`16` "NewEnumerator2" :`17` "NewEnumerator2" :`18` "NewEnumerator3" :`19` "NewEnumerator3" :`20` "NewEnumerator3" :`21` "NewEnumerator4" :`22` "NewEnumerator4" :`23` "NewEnumerator4" :`24` "NewEnumerator4" :!type "/Game/GitAssets/CJW/ETimePhase Enum")))
    (:`NewEnumerator3`
      ; 겨울
      (set `self.CurrentTimePhase` (select `int` (`self.TimeOfDay`) :`0` "NewEnumerator4" :`1` "NewEnumerator4" :`2` "NewEnumerator4" :`3` "NewEnumerator4" :`4` "NewEnumerator4" :`5` "NewEnumerator4" :`6` "NewEnumerator0" :`7` "NewEnumerator1" :`8` "NewEnumerator1" :`9` "NewEnumerator1" :`10` "NewEnumerator2" :`11` "NewEnumerator2" :`12` "NewEnumerator2" :`13` "NewEnumerator2" :`14` "NewEnumerator2" :`15` "NewEnumerator2" :`16` "NewEnumerator2" :`17` "NewEnumerator3" :`18` "NewEnumerator3" :`19` "NewEnumerator3" :`20` "NewEnumerator4" :`21` "NewEnumerator4" :`22` "NewEnumerator4" :`23` "NewEnumerator4" :`24` "NewEnumerator4" :!type "/Game/GitAssets/CJW/ETimePhase Enum")))))

(fn `TimeCal`
  (`/Engine/EditorBlueprintResources/StandardMacros.IncrementInt` (`self.TimeOfDay`)
    (:`  `
      (`|ExecutionSequence`
        (:`then_0`
          (if (>= (`self.TimeOfDay`) 25)
            (set `self.TimeOfDay` 1)
            (`self.SeasonCal`)))
        (:`then_1`
          (`self.UpdateTime`))
        (:`then_2`
          (`self.CalDayLight`))
        (:`then_3`
          (`self.SwitchTimePhase`))))))

(fn `UserConstructionScript`)