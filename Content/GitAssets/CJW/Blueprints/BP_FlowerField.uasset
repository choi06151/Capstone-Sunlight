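; Flower field actor that grows a random cluster of a chosen flower type through staged meshes, then shrinks and destroys itself.
; On BeginPlay, downward line traces scatter surface-aligned transforms around the actor.
; Two HISMs render those instances: timelines dissolve the next stage in and the current one out, then swap and repeat.
; After the final level and a delay, another timeline scales the actor down before destruction.
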(event `FirstSet`
  (bind _hism_cur (`self.HISM_Cur`))
  (`self.SetStaticMesh` _hism_cur)
  (`InstancedStaticMeshComponent.AddInstances` _hism_cur (`self.CurrentTransforms`) false true false)
  (`self.MakeFlower`))

(event `self.ReceiveBeginPlay`
  (`TimelineComponent.SetPlayRate` (`self.Timeline`) (`self.GrowthSpeed`))
  (`self.GetRandomTransforms`)
  (`self.FirstSet`))

(event `MakeFlower`
  (bind _hism_cur (`self.HISM_Cur`))
  (set `self.Level` (`KismetMathLibrary.Clamp` (+ (`self.Level`) 1) 0 13))
  (`InstancedStaticMeshComponent.ClearInstances` (`self.HISM_Nex`))
  (`self.SetStaticMesh` (`self.HISM_Nex`))
  (`InstancedStaticMeshComponent.AddInstances` (`self.HISM_Nex`) (`self.CurrentTransforms`) false true false)
  (bind (_direction _fade) (`Timeline|Timeline` :!via `PlayFromStart`)
    (:`Update`
      ; 신규
      (`MeshComponent.SetScalarParameterValueOnMaterials` (`self.HISM_Nex`) "Dissolve" (- 1.0 _fade)))
    (:`FadeOutstart`
      (bind (_direction_2 _fade_2) (`Timeline|Timeline_0` :!via `PlayFromStart`)
        (:`Update`
          ; 이전
          (`MeshComponent.SetScalarParameterValueOnMaterials` (`self.HISM_Cur`) "Dissolve" _fade_2))
        (:`Finished`
          ; 신규 0만들어 스위치 준비
          (`MeshComponent.SetScalarParameterValueOnMaterials` (`self.HISM_Nex`) "Dissolve" 0.0)
          (`InstancedStaticMeshComponent.ClearInstances` _hism_cur)
          (`self.SetStaticMesh` _hism_cur)
          (`InstancedStaticMeshComponent.AddInstances` (`self.HISM_Cur`) (`self.CurrentTransforms`) false true false)
          ; 스위치 완료
          (`MeshComponent.SetScalarParameterValueOnMaterials` (`self.HISM_Cur`) "Dissolve" 0.0)
          (if (== (`self.Level`) 13)
            (`self.StartDie`)
            (else
              (`self.MakeFlower`))))))))

(event `StartDie`
  (`KismetSystemLibrary.Delay` 5.0)
  (bind (_direction _size _fade) (`Timeline|Timeline_2` :!via `PlayFromStart`)
    (:`Update`
      (`self.SetActorScale3D` (* (1.0 1.0 1.0) (- 1.0 _fade))))
    (:`Finished`
      (`self.K2_DestroyActor`))))

(fn `GetRandomTransforms`
  (locals (MakedTransforms :type "Array of Transform Structure") (Location_Cur :type "Vector Structure"))
  (bind (_location_cur_x _location_cur_y) (`KismetMathLibrary.BreakVector` (`local.Location_Cur`)))
  (bind _returnvalue (+ (`KismetMathLibrary.MakeVector` _location_cur_x _location_cur_y 10000.0) (* (`KismetMathLibrary.RandomUnitVector`) (`KismetMathLibrary.RandomFloatInRange` 10.0 (`self.clusterRadius`)))))
  (set `local.Location_Cur` (`self.K2_GetActorLocation`))
  (for _ (range (+ (`KismetMathLibrary.RandomIntegerInRange` 1 (`self.clusterCount`)) 1))
    (bind _outhit (`KismetSystemLibrary.LineTraceSingle` _returnvalue (+ _returnvalue (0.0 0.0 -100000.0)) "TraceTypeQuery1"))
    (bind (_bblockinghit _binitialoverlap _time _distance _location _impactpoint _normal) (`GameplayStatics.BreakHitResult` _outhit))
    (if _bblockinghit
      (`KismetArrayLibrary.Array_Add` (`local.MakedTransforms`) (`KismetMathLibrary.MakeTransform` _location (`KismetMathLibrary.MakeRotFromZ` _normal) (`self.Scale`)))))
  (set `self.CurrentTransforms` (`local.MakedTransforms`))
  (return))

(fn `SetStaticMesh`
  (params (Inputmesh :type "StaticMeshComponent Object Reference"))
  (switch `/Game/GitAssets/CJW/Enum/FlowerType` (`self.Type`)
    (:`NewEnumerator0`
      (`StaticMeshComponent.SetStaticMesh` (`local.Inputmesh`) (select `int` (`self.Level`) :`0` "/Game/DriveAssets/NFlowerPack_4/Meshes/Bougainv/Bougainv_1_SM.Bougainv_1_SM" :`1` "/Game/DriveAssets/NFlowerPack_4/Meshes/Bougainv/Bougainv_2_SM.Bougainv_2_SM" :`2` "/Game/DriveAssets/NFlowerPack_4/Meshes/Bougainv/Bougainv_3_SM.Bougainv_3_SM" :`3` "/Game/DriveAssets/NFlowerPack_4/Meshes/Bougainv/Bougainv_4_SM.Bougainv_4_SM" :`4` "/Game/DriveAssets/NFlowerPack_4/Meshes/Bougainv/Bougainv_5_SM.Bougainv_5_SM" :`5` "/Game/DriveAssets/NFlowerPack_4/Meshes/Bougainv/Bougainv_6_SM.Bougainv_6_SM" :`6` "/Game/DriveAssets/NFlowerPack_4/Meshes/Bougainv/Bougainv_7_SM.Bougainv_7_SM" :`7` "/Game/DriveAssets/NFlowerPack_4/Meshes/Bougainv/Bougainv_8_SM.Bougainv_8_SM" :`8` "/Game/DriveAssets/NFlowerPack_4/Meshes/Bougainv/Bougainv_9_SM.Bougainv_9_SM" :`9` "/Game/DriveAssets/NFlowerPack_4/Meshes/Bougainv/Bougainv_10_SM.Bougainv_10_SM" :`10` "/Game/DriveAssets/NFlowerPack_4/Meshes/Bougainv/Bougainv_11_SM.Bougainv_11_SM" :`11` "/Game/DriveAssets/NFlowerPack_4/Meshes/Bougainv/Bougainv_12_SM.Bougainv_12_SM" :`12` "/Game/DriveAssets/NFlowerPack_4/Meshes/Bougainv/Bougainv_13_SM.Bougainv_13_SM" :!type "StaticMesh Object Reference")))
    (:`NewEnumerator1`
      (`StaticMeshComponent.SetStaticMesh` (`local.Inputmesh`) (select `int` (`self.Level`) :`0` "/Game/DriveAssets/NFlowerPack_4/Meshes/Dianthus/Dianthus_1_SM.Dianthus_1_SM" :`1` "/Game/DriveAssets/NFlowerPack_4/Meshes/Dianthus/Dianthus_2_SM.Dianthus_2_SM" :`2` "/Game/DriveAssets/NFlowerPack_4/Meshes/Dianthus/Dianthus_3_SM.Dianthus_3_SM" :`3` "/Game/DriveAssets/NFlowerPack_4/Meshes/Dianthus/Dianthus_4_SM.Dianthus_4_SM" :`4` "/Game/DriveAssets/NFlowerPack_4/Meshes/Dianthus/Dianthus_5_SM.Dianthus_5_SM" :`5` "/Game/DriveAssets/NFlowerPack_4/Meshes/Dianthus/Dianthus_6_SM.Dianthus_6_SM" :`6` "/Game/DriveAssets/NFlowerPack_4/Meshes/Dianthus/Dianthus_7_SM.Dianthus_7_SM" :`7` "/Game/DriveAssets/NFlowerPack_4/Meshes/Dianthus/Dianthus_8_SM.Dianthus_8_SM" :`8` "/Game/DriveAssets/NFlowerPack_4/Meshes/Dianthus/Dianthus_9_SM.Dianthus_9_SM" :`9` "/Game/DriveAssets/NFlowerPack_4/Meshes/Dianthus/Dianthus_10_SM.Dianthus_10_SM" :`10` "/Game/DriveAssets/NFlowerPack_4/Meshes/Dianthus/Dianthus_11_SM.Dianthus_11_SM" :`11` "/Game/DriveAssets/NFlowerPack_4/Meshes/Dianthus/Dianthus_12_SM.Dianthus_12_SM" :`12` "/Game/DriveAssets/NFlowerPack_4/Meshes/Dianthus/Dianthus_13_SM.Dianthus_13_SM" :!type "StaticMesh Object Reference")))
    (:`NewEnumerator2`
      (`StaticMeshComponent.SetStaticMesh` (`local.Inputmesh`) (select `int` (`self.Level`) :`0` "/Game/DriveAssets/NFlowerPack_4/Meshes/MontuakDaisy/MontuakDaisy_1_SM.MontuakDaisy_1_SM" :`1` "/Game/DriveAssets/NFlowerPack_4/Meshes/MontuakDaisy/MontuakDaisy_2_SM.MontuakDaisy_2_SM" :`2` "/Game/DriveAssets/NFlowerPack_4/Meshes/MontuakDaisy/MontuakDaisy_3_SM.MontuakDaisy_3_SM" :`3` "/Game/DriveAssets/NFlowerPack_4/Meshes/MontuakDaisy/MontuakDaisy_4_SM.MontuakDaisy_4_SM" :`4` "/Game/DriveAssets/NFlowerPack_4/Meshes/MontuakDaisy/MontuakDaisy_5_SM.MontuakDaisy_5_SM" :`5` "/Game/DriveAssets/NFlowerPack_4/Meshes/MontuakDaisy/MontuakDaisy_6_SM.MontuakDaisy_6_SM" :`6` "/Game/DriveAssets/NFlowerPack_4/Meshes/MontuakDaisy/MontuakDaisy_7_SM.MontuakDaisy_7_SM" :`7` "/Game/DriveAssets/NFlowerPack_4/Meshes/MontuakDaisy/MontuakDaisy_8_SM.MontuakDaisy_8_SM" :`8` "/Game/DriveAssets/NFlowerPack_4/Meshes/MontuakDaisy/MontuakDaisy_9_SM.MontuakDaisy_9_SM" :`9` "/Game/DriveAssets/NFlowerPack_4/Meshes/MontuakDaisy/MontuakDaisy_10_SM.MontuakDaisy_10_SM" :`10` "/Game/DriveAssets/NFlowerPack_4/Meshes/MontuakDaisy/MontuakDaisy_11_SM.MontuakDaisy_11_SM" :`11` "/Game/DriveAssets/NFlowerPack_4/Meshes/MontuakDaisy/MontuakDaisy_12_SM.MontuakDaisy_12_SM" :`12` "/Game/DriveAssets/NFlowerPack_4/Meshes/MontuakDaisy/MontuakDaisy_13_SM.MontuakDaisy_13_SM" :!type "StaticMesh Object Reference")))))

(fn `UserConstructionScript`)