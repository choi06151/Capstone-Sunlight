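; Tree field actor that morphs between cherry blossom, maple, European and bare winter trees by withering and regrowing.
; UpdateTree stores a new type, then recursive delayed events step the level down to zero, switch type and grow back at randomized, per-type timing.
; Each level swaps the mesh on an InstancedSkinnedMesh, and growth enables type-specific Niagara falling leaves from mid levels.
; Tick draws type and level as debug text.
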(event `ChangeLeaf`
  (`NiagaraComponent.SetAsset` (`self.Niagara`) (select `/Game/GitAssets/CJW/Enum/E_TreeType` (`self.TreeType`) :`NewEnumerator0` "/Game/GitAssets/CJW/VFX/NS_CherryBlossomSystem.NS_CherryBlossomSystem" :`NewEnumerator1` "/Game/GitAssets/CJW/VFX/NS_FallingLeaves_Maple.NS_FallingLeaves_Maple" :`NewEnumerator2` "/Game/GitAssets/CJW/VFX/NS_FallingLeaves_GreenLeaf.NS_FallingLeaves_GreenLeaf" :!type "NiagaraSystem Object Reference") true))

(event `CheckIsEqualTree`
  ; 몇초후 다시 검사
  (`self.DieToFirstLevel`))

(event `DieToFirstLevel`
  (if (== (`self.Level`) 0)
    (if (`|EnumInequality` (`self.NextType`) (`self.TreeType`))
      ; 새로운 시작
      (set `self.TreeType` (`self.NextType`))
      (`self.GrowToNextlevel`))
    (else
      (`/Engine/EditorBlueprintResources/StandardMacros.DecrementInt` (`self.Level`)
        (:`  `
          (`self.SetSkeletonMesh` (`self.TreeType`))
          (`KismetSystemLibrary.Delay` (`KismetMathLibrary.RandomFloatInRange` 0.0 (* (`self.TimeToGrow`) 0.5)))
          (`self.DieToFirstLevel`))))))

(event `GrowToNextlevel`
  (bind _result (`/Engine/EditorBlueprintResources/StandardMacros.IncrementInt` (`self.Level`))
    (:`  `
      (`KismetSystemLibrary.Delay` (`KismetMathLibrary.RandomFloatInRange` 0.0 (`self.TimeToGrow`)))
      (if (not (== _result 9))
        (`self.SetSkeletonMesh` (`self.TreeType`))
        (`|ExecutionSequence`
          (:`then_0`
            ; 일정량 나뭇잎이 있으면 나뭇잎 ㄹ어지게
            (if (>= (`self.Level`) 4)
              (`self.ChangeLeaf`)
              (else
                (`NiagaraComponent.SetAsset` (`self.Niagara`) null true))))
          (:`then_1`
            (`self.GrowToNextlevel`)))))))

(event `UpdateTree`
  (params (Type :type "/Game/GitAssets/CJW/Enum/E_TreeType Enum" :default "NewEnumerator0"))
  (if (`|EnumInequality` Type (`self.TreeType`))
    (set `self.NextType` Type)
    (`self.SetGrowTermAccordingToType`)
    (`self.DieToFirstLevel`)
    (else
      (set `self.TimeToGrow` (+ (`self.TimeToGrow`) 10.0)))))

(event `SetGrowTermAccordingToType`
  ; 나무마다 Term다르게
  (set `self.TimeToGrow` (* (select `/Game/GitAssets/CJW/Enum/E_TreeType` (`self.TreeType`) :`NewEnumerator0` 30.0 :`NewEnumerator1` 50.0 :`NewEnumerator2` 60.0 :`NewEnumerator3` 30.0 :`NewEnumerator4` 30.0) (`self.TimeRate`))))

(event `self.ReceiveTick`
  (params (DeltaSeconds :type "Float (single-precision)"))
  (`KismetSystemLibrary.DrawDebugString` (0.0 0.0 0.0) (`KismetStringLibrary.Concat_StrStr` (`|GetEnumeratorNameAsString` (`self.TreeType`)) (`KismetStringLibrary.Conv_IntToString` (`self.Level`))) self))

(fn `SetSkeletonMesh`
  (params (Selection :type "/Game/GitAssets/CJW/Enum/E_TreeType Enum" :default "NewEnumerator0"))
  ; cherry
  (switch `/Game/GitAssets/CJW/Enum/E_TreeType` Selection
    (:`NewEnumerator0`
      (`SkinnedMeshComponent.SetSkinnedAssetAndUpdate` (`self.InstancedSkinnedMesh`) (select `int` (`self.Level`) :`0` "/Game/DriveAssets/ForShare/CJW/Tree/CherryBlossom/Type1/CherryTree1.CherryTree1" :`1` "/Game/DriveAssets/ForShare/CJW/Tree/CherryBlossom/Type1/CherryTree2.CherryTree2" :`2` "/Game/DriveAssets/ForShare/CJW/Tree/CherryBlossom/Type1/CherryTree3.CherryTree3" :`3` "/Game/DriveAssets/ForShare/CJW/Tree/CherryBlossom/Type1/CherryTree4.CherryTree4" :`4` "/Game/DriveAssets/ForShare/CJW/Tree/CherryBlossom/Type1/CherryTree5.CherryTree5" :`5` "/Game/DriveAssets/ForShare/CJW/Tree/CherryBlossom/Type1/CherryTree6.CherryTree6" :`6` "/Game/DriveAssets/ForShare/CJW/Tree/CherryBlossom/Type1/CherryTree7.CherryTree7" :`7` "/Game/DriveAssets/ForShare/CJW/Tree/CherryBlossom/Type1/CherryTree8.CherryTree8" :`8` "/Game/DriveAssets/ForShare/CJW/Tree/CherryBlossom/Type1/CherryTree9.CherryTree9" :`9` "/Game/DriveAssets/ForShare/CJW/Tree/CherryBlossom/Type1/CherryTree10.CherryTree10" :!type "SkinnedAsset Object Reference") false))
    (:`NewEnumerator1`
      ; Maple
      (`SkinnedMeshComponent.SetSkinnedAssetAndUpdate` (`self.InstancedSkinnedMesh`) (select `int` (`self.Level`) :`0` "/Game/DriveAssets/ForShare/CJW/Tree/CherryBlossom/Type1/CherryTree1.CherryTree1" :`1` "/Game/DriveAssets/ForShare/CJW/Tree/Maple/Type1/MapleTree2.MapleTree2" :`2` "/Game/DriveAssets/ForShare/CJW/Tree/Maple/Type1/MapleTree3.MapleTree3" :`3` "/Game/DriveAssets/ForShare/CJW/Tree/Maple/Type1/MapleTree4.MapleTree4" :`4` "/Game/DriveAssets/ForShare/CJW/Tree/Maple/Type1/MapleTree5.MapleTree5" :`5` "/Game/DriveAssets/ForShare/CJW/Tree/Maple/Type1/MapleTree6.MapleTree6" :`6` "/Game/DriveAssets/ForShare/CJW/Tree/Maple/Type1/MapleTree7.MapleTree7" :`7` "/Game/DriveAssets/ForShare/CJW/Tree/Maple/Type1/MapleTree8.MapleTree8" :`8` "/Game/DriveAssets/ForShare/CJW/Tree/Maple/Type1/MapleTree9.MapleTree9" :`9` "/Game/DriveAssets/ForShare/CJW/Tree/Maple/Type1/MapleTree10.MapleTree10" :!type "SkinnedAsset Object Reference") false))
    (:`NewEnumerator2`
      ; European
      (`SkinnedMeshComponent.SetSkinnedAssetAndUpdate` (`self.InstancedSkinnedMesh`) (select `int` (`self.Level`) :`0` "/Game/DriveAssets/ForShare/CJW/Tree/CherryBlossom/Type1/CherryTree1.CherryTree1" :`1` "/Game/DriveAssets/ForShare/CJW/Tree/European2/Type1/European2.European2" :`2` "/Game/DriveAssets/ForShare/CJW/Tree/European2/Type1/European3.European3" :`3` "/Game/DriveAssets/ForShare/CJW/Tree/European2/Type1/European4.European4" :`4` "/Game/DriveAssets/ForShare/CJW/Tree/European2/Type1/European5.European5" :`5` "/Game/DriveAssets/ForShare/CJW/Tree/European2/Type1/European6.European6" :`6` "/Game/DriveAssets/ForShare/CJW/Tree/European2/Type1/European7.European7" :`7` "/Game/DriveAssets/ForShare/CJW/Tree/European2/Type1/European8.European8" :`8` "/Game/DriveAssets/ForShare/CJW/Tree/European2/Type1/European9.European9" :`9` "/Game/DriveAssets/ForShare/CJW/Tree/European2/Type1/European10.European10" :!type "SkinnedAsset Object Reference") false))
    (:`NewEnumerator4`
      (`SkinnedMeshComponent.SetSkinnedAssetAndUpdate` (`self.InstancedSkinnedMesh`) "/Game/DriveAssets/ForShare/CJW/Tree/CherryBlossom/Type1/CherryTree1.CherryTree1" true))))

(fn `UserConstructionScript`
  (set `self.TreeIdx` (`KismetMathLibrary.RandomIntegerInRange` 0 4))
  (`self.SetSkeletonMesh` "NewEnumerator0")
  (`NiagaraComponent.SetAsset` (`self.Niagara`) "/Game/GitAssets/CJW/VFX/NS_FallingLeaves_GreenLeaf.NS_FallingLeaves_GreenLeaf" true))