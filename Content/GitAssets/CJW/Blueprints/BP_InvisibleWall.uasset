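; BP_InvisibleWall is an actor that positions itself in front of BP_TempPlayer at that player's DistanceToWall.
; On BeginPlay it binds CalNewLocation to the player's distance-update event, which recomputes a cached point along the player's forward vector.
; Tick applies that cached location and sets the rotation along the player-to-wall direction, so the position only changes when the player fires the event.
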(event `self.ReceiveBeginPlay`
  (bind _asbp_temp_player (cast `/Game/GitAssets/CJW/Camera/BP_TempPlayer` (`GameplayStatics.GetPlayerCharacter` 0)))
  (bind _output_get (set `self.CameraRef` _asbp_temp_player))
  (add `/Game/DriveAssets/Cine_Cam/BP_Cine_Camera.UpdateDistanceTowall` _output_get (delegate `CalNewLocation`)))

(event `CalNewLocation`
  (bind _cameraref (`self.CameraRef`))
  (set `self.FixedLocation` (+ (* (`self.GetActorForwardVector` _cameraref) (`/Game/DriveAssets/Cine_Cam/BP_Cine_Camera.DistanceToWall` _cameraref)) (`self.K2_GetActorLocation` _cameraref))))

(event `self.ReceiveTick`
  (params (DeltaSeconds :type "Float (single-precision)"))
  (`self.K2_SetActorLocationAndRotation` (`self.FixedLocation`) (`KismetMathLibrary.FindLookAtRotation` (`self.K2_GetActorLocation` (`self.CameraRef`)) (`self.K2_GetActorLocation`))))

(fn `UserConstructionScript`)