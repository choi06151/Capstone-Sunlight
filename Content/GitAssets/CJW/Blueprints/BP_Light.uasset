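; BP_Light is a movable light actor that publishes its position to MP_ENVParameter as "PlayerPosition" and orients a plane using the player-to-light direction.
; It follows BP_HandTracker updates or timeline moves to input locations with hit effects, and can return to its origin.
; Patrol mode periodically flies via random midpoints to nearby BP_PlantSpanwer actors.
; Timers record paths into the SG_LightMovement save and replay a random saved one.
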(event `RoadHandTracker`
  (bind _returnvalue (`|SpawnActorFromClass` "/Game/GitAssets/KSJ/Leap/BP_HandTracker.BP_HandTracker_C" (`self.GetTransform`) "AdjustIfPossibleButAlwaysSpawn" "MultiplyWithRoot" null null))
  (add `/Game/GitAssets/KSJ/Leap/BP_HandTracker.UpdateLightLocation` _returnvalue (delegate `OnLightUpdate`)))

(event `OnLightUpdate`
  (params (WorldLocation :type "Vector Structure"))
  (`self.K2_SetActorLocation` (`KismetMathLibrary.VInterpTo` (`self.K2_GetActorLocation`) WorldLocation (`GameplayStatics.GetWorldDeltaSeconds`) 0.8) true))

(event `self.ReceiveBeginPlay`
  (bind _asbp_temp_player (cast `/Game/GitAssets/CJW/Camera/BP_TempPlayer` (`GameplayStatics.GetPlayerCharacter` 0)))
  (set `self.As BP Temp Player` _asbp_temp_player)
  (set `self.OriginPosition` (`self.K2_GetActorLocation`))
  (if (`self.OnHandTracking`)
    (`self.RoadHandTracker`)))

(event `StartRecordMovementInfo`
  (`KismetArrayLibrary.Array_Clear` (`self.CurrentRecordingInfo`))
  (`KismetSystemLibrary.PrintString` "녹화를 시작합니다")
  (bind _returnvalue (`KismetSystemLibrary.K2_SetTimerDelegate` (delegate `RecordMovement`) 0.01 true))
  (set `self.RecordHandler` _returnvalue))

(event `self.ReceiveTick`
  (params (DeltaSeconds :type "Float (single-precision)"))
  (bind (_returnvalue_x _returnvalue_y _returnvalue_z) (`KismetMathLibrary.BreakVector` (`self.K2_GetActorLocation`)))
  (`KismetMaterialLibrary.SetVectorParameterValue` "/Game/GitAssets/CJW/MaterialParameter/MP_ENVParameter.MP_ENVParameter" "PlayerPosition" (`KismetMathLibrary.MakeColor` _returnvalue_x _returnvalue_y _returnvalue_z))
  (`SceneComponent.K2_SetWorldRotation` (`self.Plane1`) (`KismetMathLibrary.FindLookAtRotation` (`self.K2_GetActorLocation` (`self.As BP Temp Player`)) (`self.K2_GetActorLocation`)) false false))

(event `RecordMovement`
  (`KismetArrayLibrary.Array_Add` (`self.CurrentRecordingInfo`) (`self.K2_GetActorLocation`)))

(event `StartUsingRecordingData`
  (bind (_outitem_name _outitem_moveinfo) (break `/Game/GitAssets/CJW/Record/S_LightMoveInfo` (`self.LoadRecordData`)))
  (set `self.RecordedDatas` _outitem_moveinfo)
  (set `self.RecoredIdx` 1)
  (`KismetSystemLibrary.PrintString` "녹화움직임를 시작합니다")
  (bind _returnvalue (`KismetSystemLibrary.K2_SetTimerDelegate` (delegate `MoveFollowRecordData`) 0.01 true))
  (set `self.RecordUseHandler` _returnvalue))

(event `MoveToLocation`
  (params (InputLocation :type "Vector Structure"))
  ; 마우스 컨트롤용노두
  (`|ExecutionSequence`
    (:`then_0`
      (set `self.TargetPosition` InputLocation)
      (set `self.StartPosition` (`self.K2_GetActorLocation`))
      (bind (_direction _move) (`Timeline|MoveTime` :!via `PlayFromStart`)
        (:`Update`
          (bind _sweephitresult (`self.K2_SetActorLocation` (`KismetMathLibrary.VLerp` (`self.StartPosition`) (`self.TargetPosition`) _move) true))
          (bind (_bblockinghit _binitialoverlap _time _distance _location _impactpoint _normal) (`GameplayStatics.BreakHitResult` _sweephitresult))
          (if _bblockinghit
            (`NiagaraFunctionLibrary.SpawnSystemAtLocation` "/Game/GitAssets/CJW/VFX/HitVFx/NS_Hit.NS_Hit" _location (`KismetMathLibrary.MakeRotFromX` _normal) (0.1 0.1 0.1))))))
    (:`then_1`
      (`/Engine/EditorBlueprintResources/StandardMacros.DoOnce` false :!label _label
        (:`Completed`
          (bind (_direction_2 _newtrack_0) (`Timeline|BackTimeline` :!via `Stop` :!label _label_2)
            (:`Update`
              (`self.K2_SetActorLocation` (`KismetMathLibrary.VLerp` (`self.StartPosition`) (`self.OriginPosition`) _newtrack_0) true))))))))

(event `MoveFollowRecordData`
  (bind _recoredidx (`self.RecoredIdx`))
  (bind _recordeddatas (`self.RecordedDatas`))
  (`self.K2_SetActorLocation` (`KismetMathLibrary.VInterpTo` (`|GetArrayItem` _recordeddatas (- _recoredidx 1)) (`|GetArrayItem` _recordeddatas _recoredidx) (`GameplayStatics.GetWorldDeltaSeconds`) 20.0))
  (`/Engine/EditorBlueprintResources/StandardMacros.IncrementInt` (`self.RecoredIdx`)
    (:`  `
      (if (>= (`self.RecoredIdx`) (`KismetArrayLibrary.Array_Length` (`self.RecordedDatas`)))
        (`KismetSystemLibrary.K2_PauseTimerHandle` (`self.RecordUseHandler`))))))

(event `StartPatrolFlowerMode`
  (`self.PatrolToInteractFlower`)
  (bind _returnvalue (`KismetSystemLibrary.K2_SetTimerDelegate` (delegate `PatrolToInteractFlower`) 30.0 true))
  (set `self.PatrolHandler` _returnvalue))

(event `PatrolToInteractFlower`
  (bind _targetposition (`self.TargetPosition`))
  (`|ExecutionSequence`
    (:`then_0`
      (set `self.StartPosition` (`self.K2_GetActorLocation`))
      (set `self.TargetPosition` (+ (`self.GetMovePointAroundMiddlePoint`) (0.0 0.0 100.0)))
      (set `self.MiddlePosition` (+ (/ (+ (`self.StartPosition`) (`self.TargetPosition`)) 2.0) (* (`KismetMathLibrary.RandomUnitVector`) 4.0)))
      (bind (_direction _newtrack_0) (`Timeline|Move1` :!via `PlayFromStart`)
        (:`Update`
          (`self.K2_SetActorLocation` (`KismetMathLibrary.VLerp` (`self.StartPosition`) (`self.MiddlePosition`) _newtrack_0)))
        (:`Finished`
          (bind (_direction_2 _newtrack_0_2) (`Timeline|Move2` :!via `PlayFromStart`)
            (:`Update`
              (`self.K2_SetActorLocation` (`KismetMathLibrary.VLerp` (`self.MiddlePosition`) (`self.TargetPosition`) _newtrack_0_2)))
            (:`Finished`
              (`Timeline|ShakeTimeline` :!label _label_3
                (:`Update`
                  (`self.K2_SetActorLocation` (`KismetMathLibrary.VInterpTo` _targetposition (`NavigationSystemV1.K2_GetRandomReachablePointInRadius` _targetposition 50.0 null null) (`GameplayStatics.GetWorldDeltaSeconds`) 0.0001)))))))))
    (:`then_1`
      (goto _label_3 :!via `Stop`))))

(event `MoveToOriginPlace`
  ; 마우스 컨트롤용노두
  (`|ExecutionSequence`
    (:`then_0`
      (set `self.StartPosition` (`self.K2_GetActorLocation`))
      (goto _label_2 :!via `PlayFromStart`))
    (:`then_1`
      (goto _label :!via `Reset`))))

(fn `ClearRecords`
  (bind _returnvalue (`GameplayStatics.LoadGameFromSlot` "SavedMoveInfo"))
  (bind _assg_light_movement (cast `/Game/GitAssets/CJW/Record/SG_LightMovement` _returnvalue))
  (`KismetArrayLibrary.Array_Clear` (`/Game/GitAssets/CJW/Record/SG_LightMovement.SavedMovementInfo` _assg_light_movement))
  (`KismetSystemLibrary.PrintString` "기존의 기록을 삭제합니다")
  (`GameplayStatics.SaveGameToSlot` _returnvalue "SavedMoveInfo"))

(fn `GetMovePointAroundMiddlePoint`
  (returns (ReturnValue :type "Vector Structure"))
  (locals (Points :type "Array of Actor Object Reference"))
  (bind _points (`local.Points`))
  (bind _returnvalue (`self.K2_GetActorLocation` (`self.MiddlePoint`)))
  (bind _output (`|GetArrayItem` _points (`KismetMathLibrary.RandomIntegerInRange` 0 (- (`KismetArrayLibrary.Array_Length` _points) 1))))
  (bind _outhits (`KismetSystemLibrary.SphereTraceMultiForObjects` :`Start` _returnvalue :`End` _returnvalue :`Radius` 1500.0 :`ObjectTypes` (`|MakeArray` "ObjectTypeQuery2" :!type "EObjectTypeQuery Enum") :`DrawDebugType` "ForDuration"))
  (for _array_element _outhits
    (bind (_bblockinghit _binitialoverlap _time _distance _location _impactpoint _normal _impactnormal _physmat _hitactor) (`GameplayStatics.BreakHitResult` _array_element))
    (cast `/Game/GitAssets/CJW/Blueprints/Flower/BP_PlantSpanwer` _hitactor)
    (`KismetArrayLibrary.Array_Add` (`local.Points`) _hitactor))
  (`/Engine/EditorBlueprintResources/StandardMacros.IsValid` _output
    (:`Is Valid`
      (return (+ (`self.K2_GetActorLocation` _output) (0.0 0.0 100.0))))
    (:`Is Not Valid`
      (return (+ (`self.K2_GetActorLocation` (`self.MiddlePoint`)) (0.0 0.0 100.0))))))

(fn `LoadRecordData`
  (returns (OutItem :type "/Game/GitAssets/CJW/Record/S_LightMoveInfo Structure"))
  (bind _returnvalue (`GameplayStatics.LoadGameFromSlot` "SavedMoveInfo"))
  (bind _assg_light_movement (cast `/Game/GitAssets/CJW/Record/SG_LightMovement` _returnvalue))
  (return (`KismetArrayLibrary.Array_Random` (`/Game/GitAssets/CJW/Record/SG_LightMovement.SavedMovementInfo` _assg_light_movement))))

(fn `PauseRecordMovement`
  (bind _s_lightmoveinfo (make `/Game/GitAssets/CJW/Record/S_LightMoveInfo` (`self.RecordingName`) (`self.CurrentRecordingInfo`)))
  (`KismetSystemLibrary.K2_PauseTimerHandle` (`self.RecordHandler`))
  (`KismetSystemLibrary.PrintString` "녹화를 종료합니다")
  (bind _returnvalue (`GameplayStatics.DoesSaveGameExist` "SavedMoveInfo"))
  (if _returnvalue
    (bind _returnvalue_2 (`GameplayStatics.LoadGameFromSlot` "SavedMoveInfo"))
    (bind _assg_light_movement (cast `/Game/GitAssets/CJW/Record/SG_LightMovement` _returnvalue_2))
    (`KismetArrayLibrary.Array_Add` (`/Game/GitAssets/CJW/Record/SG_LightMovement.SavedMovementInfo` _assg_light_movement) _s_lightmoveinfo)
    (`GameplayStatics.SaveGameToSlot` _returnvalue_2 "SavedMoveInfo")
    (else
      (bind _returnvalue_3 (`GameplayStatics.CreateSaveGameObject` "/Game/GitAssets/CJW/Record/SG_LightMovement.SG_LightMovement_C"))
      (`KismetArrayLibrary.Array_Add` (`/Game/GitAssets/CJW/Record/SG_LightMovement.SavedMovementInfo` _returnvalue_3) _s_lightmoveinfo)
      (`GameplayStatics.SaveGameToSlot` _returnvalue_3 "SavedMoveInfo"))))

(fn `UserConstructionScript`
  (bind (_returnvalue_x _returnvalue_y _returnvalue_z) (`KismetMathLibrary.BreakVector` (`self.K2_GetActorLocation`)))
  (`KismetMaterialLibrary.SetVectorParameterValue` "/Game/GitAssets/CJW/MaterialParameter/MP_ENVParameter.MP_ENVParameter" "PlayerPosition" (`KismetMathLibrary.MakeColor` _returnvalue_x _returnvalue_y _returnvalue_z)))