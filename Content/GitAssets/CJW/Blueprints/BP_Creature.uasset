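; BP_Creature is an animated flower creature that cycles through geometry-cache clips and reacts to sphere overlaps.
; From BeginPlay, the self-calling Glow event advances Level, plays the matching Flower_part cache, waits its duration, then repeats, wrapping before the last part.
; Sphere overlap resumes playback, while leaving stops it and starts a Delay timeline that reverses the cache when finished.
; Tick draws a debug sphere around the actor.
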(event `self.ReceiveBeginPlay`
  (`GameplayStatics.SetGlobalTimeDilation` 1.0)
  (`self.Glow`))

(event `Glow`
  (bind _geometrycache (`self.GeometryCache`))
  (bind _output_get (set `self.Level` (`KismetMathLibrary.Clamp` (+ (`self.Level`) 1) 0 7)))
  (if (== _output_get 7)
    (set `self.Level` -1)
    (`self.Glow`)
    (else
      (`GeometryCacheComponent.SetGeometryCache` _geometrycache (select `int` (`self.Level`) :`0` "/Game/DriveAssets/ForShare/CJW/Flower/Caches/flower_part_1.flower_part_1" :`1` "/Game/DriveAssets/ForShare/CJW/Flower/Caches/flower_part_2.flower_part_2" :`2` "/Game/DriveAssets/ForShare/CJW/Flower/Caches/flower_part_3.flower_part_3" :`3` "/Game/DriveAssets/ForShare/CJW/Flower/Caches/flower_part_4.flower_part_4" :`4` "/Game/DriveAssets/ForShare/CJW/Flower/Caches/flower_part_5.flower_part_5" :`5` "/Game/DriveAssets/ForShare/CJW/Flower/Caches/flower_part_6.flower_part_6" :`6` "/Game/DriveAssets/ForShare/CJW/Flower/Caches/flower_part_7.flower_part_7" :`7` "/Game/DriveAssets/ForShare/CJW/Flower/Caches/flower_part_8.flower_part_8" :!type "GeometryCache Object Reference"))
      (`GeometryCacheComponent.PlayFromStart` _geometrycache)
      (`KismetSystemLibrary.Delay` (`GeometryCacheComponent.GetDuration` (`self.GeometryCache`)))
      (`self.Glow`))))

(event `self.ReceiveActorBeginOverlap`
  (params (OtherActor :type "Actor Object Reference")))

(event `self.ReceiveTick`
  (params (DeltaSeconds :type "Float (single-precision)"))
  (`KismetSystemLibrary.DrawDebugSphere` (`self.K2_GetActorLocation`) 150.0 12 (struct :`R` 1.0 :`G` 1.0 :`B` 1.0 :`A` 1.0) 0.1))

(event `self.Sphere.OnComponentBeginOverlap`
  (params (OverlappedComponent :type "PrimitiveComponent Object Reference") (OtherActor :type "Actor Object Reference") (OtherComp :type "PrimitiveComponent Object Reference") (OtherBodyIndex :type Integer) (bFromSweep :type Boolean) (SweepResult :type "HitResult Structure (by ref)"))
  (`GeometryCacheComponent.Play` (`self.GeometryCache`)))

(event `self.Sphere.OnComponentEndOverlap`
  (params (OverlappedComponent :type "PrimitiveComponent Object Reference") (OtherActor :type "Actor Object Reference") (OtherComp :type "PrimitiveComponent Object Reference") (OtherBodyIndex :type Integer))
  (`GeometryCacheComponent.Stop` (`self.GeometryCache`))
  (`self.StartShrink`))

(event `StartShrink`
  (`Timeline|Delay` :!via `PlayFromStart`
    (:`Finished`
      (`GeometryCacheComponent.PlayReversed` (`self.GeometryCache`)))))

(fn `UserConstructionScript`)