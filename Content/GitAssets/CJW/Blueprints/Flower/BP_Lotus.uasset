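; Lotus plant actor that grows through geometry-cache stages while a BP_Light overlaps its sphere.
; A detection timeline advances leaf stages to the head bloom and turns the head toward the light.
; Losing the light stops playback, then a delay timeline reverses the current cache until light returns.
; Full bloom triggers success VFX and sound and notifies the owning BP_PlantSpanwer, while StartDIe scales the plant away after a random delay.
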(event `Plant`
  ; 늦봄 ~ 초여름
  (set `self.Level` 0)
  (`GeometryCacheComponent.SetGeometryCache` (`self.Leaf`) (select `int` (`self.Level`) :`0` "/Game/DriveAssets/ForShare/CJW/Flower/Lotus/Caches/Lotus_rhizome_all1_0.Lotus_rhizome_all1_0" :`1` "/Game/DriveAssets/ForShare/CJW/Flower/Peony/Caches/flower_new_part2.flower_new_part2" :!type "GeometryCache Object Reference")))

(event `self.ReceiveBeginPlay`
  (`self.Plant`))

(event `Glow`
  (bind _leaf (`self.Leaf`))
  (`|ExecutionSequence`
    (:`then_1`
      (bind _output_get (set `self.Level` (`KismetMathLibrary.Clamp` (+ (`self.Level`) 1) 0 2)))
      (if (== _output_get 2)
        (`GeometryCacheComponent.SetGeometryCache` (`self.Head`) (select `int` (`self.Level`) :`0` null :`1` null :`2` "/Game/DriveAssets/ForShare/CJW/Flower/Lotus/Caches/Lotus_rhizome_all3_0.Lotus_rhizome_all3_0" :!type "GeometryCache Object Reference"))
        (bind (_direction _scale) (`Timeline|GlowFlower` :!label _label)
          (:`Update`
            (`SceneComponent.SetRelativeScale3D` (`self.Head`) _scale)
            (if (not (`GeometryCacheComponent.IsPlaying` (`self.Head`)))
              (set `self.IsFullGrow` true)
              (`NiagaraFunctionLibrary.SpawnSystemAtLocation` "/Game/GitAssets/CJW/VFX/Flower/NS_SuccessGrowth.NS_SuccessGrowth" (`self.K2_GetActorLocation`) (struct) (0.05 0.05 0.05))
              (`ActorComponent.Deactivate` (`self.NS_Growing`))
              (`GameplayStatics.PlaySoundAtLocation` "/Game/DriveAssets/sounds/flowerfinish.flowerfinish" (`self.K2_GetActorLocation`) (struct) 1.0 1.0 0.0 "/Game/GitAssets/CJW/SoundSetting/SA_Animal.SA_Animal" null null null)
              (`AudioComponent.SetVolumeMultiplier` (`self.FlowerGrow`) 0.0)
              (bind _asbp_plant_spanwer (cast `/Game/GitAssets/CJW/Blueprints/Flower/BP_PlantSpanwer` (`self.GetOwner`)))
              (`/Game/GitAssets/CJW/Blueprints/Flower/BP_PlantSpanwer.OffVFX` _asbp_plant_spanwer)
              (`Timeline|PlayDetect` :!label _label_2
                (:`Update`
                  (`|ExecutionSequence`
                    (:`then_0`
                      (if (`GeometryCacheComponent.IsPlaying` (`self.Leaf`))
                        _
                        (elif (`self.IsFullGrow`)
                          (set `self.Level` 3)
                          (else
                            (`self.Glow`)))))
                    (:`then_1`
                      (if (not (`self.IsFullGrow`))
                        (`self.SetRotation`)))))))))
        (else
          (`GeometryCacheComponent.SetGeometryCache` _leaf (select `int` (`self.Level`) :`0` "/Game/DriveAssets/ForShare/CJW/Flower/Lotus/Caches/Lotus_rhizome_all1_0.Lotus_rhizome_all1_0" :`1` "/Game/DriveAssets/ForShare/CJW/Flower/Lotus/Caches/Lotus_rhizome_all2_0.Lotus_rhizome_all2_0" :!type "GeometryCache Object Reference"))
          (`GeometryCacheComponent.PlayFromStart` _leaf)
          (goto _label_2))))))

(event `self.ReceiveActorBeginOverlap`
  (params (OtherActor :type "Actor Object Reference")))

(event `SetRotation`
  (`SceneComponent.K2_SetWorldRotation` (`self.Head`) (`KismetMathLibrary.MakeRotFromZ` (`KismetMathLibrary.Normal` (- (`self.K2_GetActorLocation` (`self.Light`)) (`SceneComponent.K2_GetComponentLocation` (`self.Head`))))) false false))

(event `self.ReceiveTick`
  (params (DeltaSeconds :type "Float (single-precision)")))

(event `self.Sphere.OnComponentBeginOverlap`
  (params (OverlappedComponent :type "PrimitiveComponent Object Reference") (OtherActor :type "Actor Object Reference") (OtherComp :type "PrimitiveComponent Object Reference") (OtherBodyIndex :type Integer) (bFromSweep :type Boolean) (SweepResult :type "HitResult Structure (by ref)"))
  (cast `/Game/GitAssets/CJW/Blueprints/BP_Light` OtherActor)
  (set `self.Light` OtherActor)
  (if (not (`self.IsFullGrow`))
    (`AudioComponent.SetVolumeMultiplier` (`self.FlowerGrow`) 0.2)
    (`ActorComponent.Activate` (`self.NS_Growing`) false)
    (`GeometryCacheComponent.Play` (`self.Leaf`))
    (`GeometryCacheComponent.Play` (`self.Head`))
    (`|ExecutionSequence`
      (:`then_0`
        (goto _label_2))
      (:`then_1`
        (`Timeline|Delay` :!via `Stop` :!label _label_3
          (:`Finished`
            (if (>= (`self.Level`) 2)
              (`GeometryCacheComponent.PlayReversed` (`self.Head`))
              (else
                (`GeometryCacheComponent.PlayReversed` (`self.Leaf`))))))))))

(event `self.Sphere.OnComponentEndOverlap`
  (params (OverlappedComponent :type "PrimitiveComponent Object Reference") (OtherActor :type "Actor Object Reference") (OtherComp :type "PrimitiveComponent Object Reference") (OtherBodyIndex :type Integer))
  (cast `/Game/GitAssets/CJW/Blueprints/BP_Light` OtherActor)
  (set `self.Light` null)
  (`AudioComponent.SetVolumeMultiplier` (`self.FlowerGrow`) 0.0)
  (`ActorComponent.Deactivate` (`self.NS_Growing`))
  (`|ExecutionSequence`
    (:`then_0`
      (`GeometryCacheComponent.Stop` (`self.Leaf`))
      (`GeometryCacheComponent.Stop` (`self.Head`))
      (goto _label_2 :!via `Stop`))
    (:`then_1`
      (`self.StartShrink`))
    (:`then_2`
      (goto _label :!via `Stop`))))

(event `StartShrink`
  (if (!= (`self.Level`) 3)
    (goto _label_3 :!via `PlayFromStart`)))

(event `/Game/GitAssets/CJW/Interface/FlowerInterface.StartDIe`
  (`KismetSystemLibrary.Delay` (`KismetMathLibrary.RandomFloatInRange` 5.0 150.0))
  (bind (_direction _newtrack_0) (`Timeline|Timeline` :!via `PlayFromStart`)
    (:`Update`
      (`self.SetActorScale3D` (`KismetMathLibrary.Conv_DoubleToVector` (`KismetMathLibrary.Lerp` 1.0 0.0 _newtrack_0))))))

(fn `UserConstructionScript`)