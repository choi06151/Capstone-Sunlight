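; BP_PlantSpanwer is an actor that spawns one flower of a chosen type at its own transform.
; SetNewFlower destroys the current plant, then spawns the Blueprint matching the type enum, such as Peony, Tulip, Prennis, Lotus or CornPoppy.
; After a spawn, the NSItsFlowerExsist effect activates following a random delay of a few seconds.
; A Nothing type or the OffVFX event deactivates that effect.
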(event `SetNewFlower`
  (params (Type :type "/Game/GitAssets/CJW/Enum/E_InteractFlower Enum" :default "NewEnumerator0"))
  (set `self.CurrentType` Type)
  (bind _spawnedplant (`self.SpawnedPlant`)
    (:`then`
      (`self.K2_DestroyActor` _spawnedplant))
    (:`else`
      _))
  (if (`|EnumInequality` (`self.CurrentType`) "NewEnumerator0")
    (bind _returnvalue (`|SpawnActorFromClass` (select `/Game/GitAssets/CJW/Enum/E_InteractFlower` (`self.CurrentType`) :`NewEnumerator0` "/Game/GitAssets/CJW/Blueprints/Flower/BP_Tulip.BP_Tulip_C" :`NewEnumerator1` "/Game/GitAssets/CJW/Blueprints/Flower/BP_Peony.BP_Peony_C" :`NewEnumerator2` "/Game/GitAssets/CJW/Blueprints/Flower/BP_Tulip.BP_Tulip_C" :`NewEnumerator3` "/Game/GitAssets/CJW/Blueprints/Flower/BP_Prennis.BP_Prennis_C" :`NewEnumerator4` "/Game/GitAssets/CJW/Blueprints/Flower/BP_Lotus.BP_Lotus_C" :`NewEnumerator5` "/Game/GitAssets/CJW/Blueprints/Flower/BP_CornPoppy.BP_CornPoppy_C" :!type "Actor Class Reference") (`self.GetTransform`) "AlwaysSpawn" "MultiplyWithRoot" self null))
    (set `self.SpawnedPlant` _returnvalue)
    (`KismetSystemLibrary.Delay` (`KismetMathLibrary.RandomFloatInRange` 0.0 5.0))
    (`ActorComponent.Activate` (`self.NS_ItsFlowerExsist`) false)
    (else
      (`ActorComponent.Deactivate` (`self.NS_ItsFlowerExsist`) :!label _label))))

(event `self.ReceiveBeginPlay`)

(event `OffVFX`
  (goto _label))

(fn `UserConstructionScript`)