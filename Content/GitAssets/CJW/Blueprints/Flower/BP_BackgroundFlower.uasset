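; Background flower actor whose skinned mesh reflects a level, from empty through several flower stages.
; SetFlower stores the level and swaps the mesh after a random delay of a few seconds.
; SwingTree plays a timeline that wobbles roll and pitch within random bounds re-rolled each update.
; The timeline's Left output restores the starting rotation and spawns a butterfly particle above flowers at level three or higher.
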(event `SetFlower`
  (params (Level :type Integer))
  (set `self.Level` Level)
  (`KismetSystemLibrary.Delay` (`KismetMathLibrary.RandomFloatInRange` 0.0 5.0))
  (`SkinnedMeshComponent.SetSkinnedAssetAndUpdate` (`self.InstancedSkinnedMesh`) (select `int` Level :`0` "/Game/DriveAssets/ForShare/CJW/BackgroundFlower/FlowerEmpty.FlowerEmpty" :`1` "/Game/DriveAssets/ForShare/CJW/BackgroundFlower/Flower1.Flower1" :`2` "/Game/DriveAssets/ForShare/CJW/BackgroundFlower/Flower2.Flower2" :`3` "/Game/DriveAssets/ForShare/CJW/BackgroundFlower/Rose/RoseFlower3.RoseFlower3" :`4` "/Game/DriveAssets/ForShare/CJW/BackgroundFlower/Rose/RoseFlower4.RoseFlower4" :`5` "/Game/DriveAssets/ForShare/CJW/BackgroundFlower/Rose/RoseFlower5.RoseFlower5" :!type "SkinnedAsset Object Reference") false))

(event `SwingTree`
  (bind (_first_rotation_roll _first_rotation_pitch _first_rotation_yaw) (`KismetMathLibrary.BreakRotator` (`self.First Rotation`)))
  (set `self.First Rotation` (`self.K2_GetActorRotation`))
  (bind (_direction _lerp) (`Timeline|Timeline` :!via `PlayFromStart`)
    (:`Update`
      (`self.K2_SetActorRotation` (`KismetMathLibrary.RLerp` (`KismetMathLibrary.MakeRotator` (+ _first_rotation_roll (`KismetMathLibrary.RandomFloatInRange` -2.0)) (+ _first_rotation_pitch (`KismetMathLibrary.RandomFloatInRange` -2.0)) _first_rotation_yaw) (`KismetMathLibrary.MakeRotator` (+ _first_rotation_roll (`KismetMathLibrary.RandomFloatInRange` 0.0 2.0)) (+ _first_rotation_pitch (`KismetMathLibrary.RandomFloatInRange` 0.0 2.0)) _first_rotation_yaw) _lerp)))
    (:`Left`
      (`self.K2_SetActorRotation` (`self.First Rotation`))
      (if (>= (`self.Level`) 3)
        (`GameplayStatics.SpawnEmitterAtLocation` "/Game/Realistic_Starter_VFX_Pack_Vol2/Particles/Environment/P_Butterfly.P_Butterfly" (+ (`self.K2_GetActorLocation`) (0.0 0.0 100.0)) (struct) (0.2 0.2 0.2))))))

(fn `UserConstructionScript`)