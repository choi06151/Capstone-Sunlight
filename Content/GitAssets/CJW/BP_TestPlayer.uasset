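; BP_TestPlayer is a test player that drives environment controls and a movable light from keyboard keys.
; On BeginPlay it creates the WBP_Test widget and finds the BP_Light actor.
; V/B/N/M switch environments through the widget, while 9/0 control global time and 4 sets random snow through the widget's environment reference.
; Key 8 toggles a mode where a looping timer traces under the cursor and moves the light to the hit.
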(event `self.ReceiveBeginPlay`
  (`parent.ReceiveBeginPlay`)
  (bind _returnvalue (`|CreateWidget` "/Game/GitAssets/CJW/WBP_Test.WBP_Test_C"))
  (bind _output_get (set `self.Ref_WBP_Test` _returnvalue))
  (`UserWidget.AddToViewport` _output_get 0)
  (bind _returnvalue_2 (`GameplayStatics.GetActorOfClass` "/Game/GitAssets/CJW/Blueprints/BP_Light.BP_Light_C"))
  (set `self.Ref_BP_Light` _returnvalue_2))

(event `Key|Eight`
  (params (Key :type "Key Structure"))
  (bind _returnvalue (`GameplayStatics.GetPlayerController` 0))
  (bind _returnvalue_2 (`GameplayStatics.GetPlayerController` 0))
  (:`Pressed`
    (`|ExecutionSequence`
      (:`then_0`
        (set `self.MovingLightMode` (not (`self.MovingLightMode`)))
        (`self.UpdateInfo`))
      (:`then_1`
        (if (`self.MovingLightMode`)
          (`WidgetBlueprintLibrary.SetInputMode_GameAndUIEx` _returnvalue (`self.Ref_WBP_Test`) "LockAlways")
          (set `PlayerController.bShowMouseCursor` false _returnvalue)
          (bind _returnvalue_3 (`KismetSystemLibrary.K2_SetTimerDelegate` (delegate `ShotLineTrace`) 0.1 true))
          (set `self.CursurBehaviorTimer` _returnvalue_3)
          (else
            (`WidgetBlueprintLibrary.SetInputMode_GameOnly` _returnvalue_2 true)
            (set `PlayerController.bShowMouseCursor` false _returnvalue_2)
            (`KismetSystemLibrary.K2_PauseTimerHandle` (`self.CursurBehaviorTimer`))))))))

(event `Key|V`
  (params (Key :type "Key Structure"))
  (:`Pressed`
    (`/Game/GitAssets/CJW/WBP_Test.ChangeENV` (`self.Ref_WBP_Test`) "NewEnumerator0")))

(event `Key|B`
  (params (Key :type "Key Structure"))
  (:`Pressed`
    (`/Game/GitAssets/CJW/WBP_Test.ChangeENV` (`self.Ref_WBP_Test`) "NewEnumerator1")))

(event `Key|N`
  (params (Key :type "Key Structure"))
  (:`Pressed`
    (`/Game/GitAssets/CJW/WBP_Test.ChangeENV` (`self.Ref_WBP_Test`) "NewEnumerator2")))

(event `ShotLineTrace`
  (bind (_bblockinghit _binitialoverlap _time _distance _location) (`GameplayStatics.BreakHitResult` (`PlayerController.GetHitResultUnderCursorByChannel` (`GameplayStatics.GetPlayerController` 0) "TraceTypeQuery3" true)))
  (if _bblockinghit
    (`/Game/GitAssets/CJW/Blueprints/BP_Light.MoveToLocation` (`self.Ref_BP_Light`) _location)))

(event `Key|M`
  (params (Key :type "Key Structure"))
  (:`Pressed`
    (`/Game/GitAssets/CJW/WBP_Test.ChangeENV` (`self.Ref_WBP_Test`) "NewEnumerator3")))

(event `Key|Nine`
  (params (Key :type "Key Structure"))
  (bind _ref_wbp_test (`self.Ref_WBP_Test`))
  (:`Pressed`
    (`/Game/GitAssets/CJW/Blueprints/BP_ENV.ControlGlobalTime` (`/Game/GitAssets/CJW/WBP_Test.BP_ENV_Ref` _ref_wbp_test) false)
    (`/Game/GitAssets/CJW/WBP_Test.UpdateTime_Event` _ref_wbp_test :!label _label)))

(event `Key|Zero`
  (params (Key :type "Key Structure"))
  (:`Pressed`
    (`/Game/GitAssets/CJW/Blueprints/BP_ENV.ControlGlobalTime` (`/Game/GitAssets/CJW/WBP_Test.BP_ENV_Ref` (`self.Ref_WBP_Test`)) true)
    (goto _label)))

(event `Key|Four`
  (params (Key :type "Key Structure"))
  (:`Pressed`
    (`/Game/GitAssets/CJW/Blueprints/BP_ENV.ControlSnow` (`/Game/GitAssets/CJW/WBP_Test.BP_ENV_Ref` (`self.Ref_WBP_Test`)) (`KismetMathLibrary.RandomIntegerInRange` 0 4))))

(fn `UserConstructionScript`
  (`parent.UserConstructionScript`))