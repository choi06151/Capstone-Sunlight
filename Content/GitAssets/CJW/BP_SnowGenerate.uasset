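; Geometry Script generated mesh actor that procedurally builds a snow layer over the actors in MeshesToAddSnowToo.
; On rebuild it merges their meshes, builds a BVH, and appends small spheres where randomly placed, seeded downward rays hit.
; The result moves to actor space, with optional Remesh applying morphology thickness, smoothing, box UVs, tangents and normals.
; At runtime, a bound value-change event triggers an immediate rebuild every 50th call.
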(event `self.ReceiveBeginPlay`
  (add `self.ValueChange` (delegate `RefreshMesh`)))

(event `RefreshMesh`
  (bind _filtercount (`self.filterCount`))
  (`/Engine/EditorBlueprintResources/StandardMacros.IncrementInt` _filtercount
    (:`  `
      (if (>= _filtercount 50)
        (set `self.filterCount` 0)
        (`self.MarkForMeshRebuild` true)))))

(event `self.OnRebuildGeneratedMesh`
  (params (TargetMesh :type "DynamicMesh Object Reference"))
  (bind _stream (`self.Stream`))
  (set `self.Target Mesh` TargetMesh)
  (`|ExecutionSequence`
    (:`then_0`
      (bind _returnvalue (`self.AllocateComputeMesh`))
      (set `self.RaycastMeshActors` _returnvalue)
      (for _array_element (`self.MeshesToAddSnowToo`)
        (bind _returnvalue_2 (`self.AllocateComputeMesh`))
        (bind (_localtoworld _returnvalue_3) (`GeometryScriptLibrary_SceneUtilityFunctions.CopyMeshFromComponent` (`Actor.RootComponent` _array_element) _returnvalue_2 (struct) true)
          (:`Failure`
            (`KismetSystemLibrary.PrintString` "fail"))
          (:`Success`
            (`GeometryScriptLibrary_MeshBasicEditFunctions.AppendMesh` (`self.RaycastMeshActors`) _returnvalue_3 (struct) false (struct :`CombineMode` "EnableAllMatching"))))
        (`self.ReleaseComputeMesh` _returnvalue_2)))
    (:`then_1`
      (bind (_outputbvh _returnvalue_4) (`GeometryScriptLibrary_MeshSpatial.BuildBVHForMesh` (`self.RaycastMeshActors`)))
      (set `self.Output BVH` _outputbvh)
      (for _ (range (+ (`self.NumberOfSphere`) 1))
        (bind _returnvalue_5 (`GeometryScriptLibrary_MeshQueryFunctions.GetMeshBoundingBox` _returnvalue_4))
        (bind _hitresult (`GeometryScriptLibrary_MeshSpatial.FindNearestRayIntersectionWithMesh` (`self.RaycastMeshActors`) (`self.Output BVH`) (`KismetMathLibrary.MakeVector` (`KismetMathLibrary.RandomFloatInRangeFromStream` _stream (.x (break `Box` _returnvalue_5)) (.x (`.Max` (break `Box` _returnvalue_5)))) (`KismetMathLibrary.RandomFloatInRangeFromStream` _stream (.y (break `Box` _returnvalue_5)) (.y (`.Max` (break `Box` _returnvalue_5)))) (+ (- (.z (break `Box` _returnvalue_5)) (.z (`.Max` (break `Box` _returnvalue_5)))) 1000.0)) (0.0 0.0 -1.0))
          (:`Found`
            (`GeometryScriptLibrary_MeshPrimitiveFunctions.AppendSphereBox` (`self.Target Mesh`) (struct) (`KismetMathLibrary.MakeTransform` (`.HitPosition` (break `GeometryScriptRayHitResult` _hitresult))) 5.0)))))
    (:`then_2`
      (`GeometryScriptLibrary_MeshTransformFunctions.TransformMesh` (`self.Target Mesh`) (`KismetMathLibrary.InvertTransform` (`self.GetTransform`))))
    (:`then_3`
      (if (`self.Remesh`)
        (bind _returnvalue_6 (`GeometryScriptLibrary_MeshVoxelFunctions.ApplyMeshMorphology` (`self.Target Mesh`) (make `GeometryScriptMorphologyOptions` (make `GeometryScript3DGridParameters` "GridResolution") false (make `GeometryScript3DGridParameters` "GridResolution") (struct :`Min` (0.0 0.0 0.0) :`Max` (0.0 0.0 0.0)) "Dilate" (`self.SnowThickness`))))
        (`GeometryScriptLibrary_MeshDeformFunctions.ApplyIterativeSmoothingToMesh` _returnvalue_6 (struct) (make `GeometryScriptIterativeMeshSmoothingOptions` (`self.SmoothIterations`)))
        (bind (_returnvalue_min _returnvalue_max) (break `Box` (`GeometryScriptLibrary_MeshQueryFunctions.GetMeshBoundingBox` _returnvalue_6)))
        (bind _returnvalue_7 (`GeometryScriptLibrary_MeshUVFunctions.SetMeshUVsFromBoxProjection` _returnvalue_6 0 (`KismetMathLibrary.MakeTransform` (0.0 0.0 0.0) (struct) (- _returnvalue_max _returnvalue_min))))
        (bind _returnvalue_8 (`GeometryScriptLibrary_MeshNormalsFunctions.ComputeTangents` _returnvalue_7))
        (`GeometryScriptLibrary_MeshNormalsFunctions.ComputeSplitNormals` _returnvalue_8 (make `GeometryScriptSplitNormalsOptions` true 80.0))))
    (:`then_4`
      (`self.ReleaseAllComputeMeshes`))))

(fn `UserConstructionScript`)