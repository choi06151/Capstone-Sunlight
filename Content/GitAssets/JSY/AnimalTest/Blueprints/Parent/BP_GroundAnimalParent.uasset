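; Parent Blueprint for ground animal characters that wander around a middle point, react to touch and eventually leave.
; BeginPlay caches tagged TargetPoints, and MoveToMiddle starts a recursive AIMoveTo patrol across random reachable points.
; Clicks or "HandTouch" overlaps stop the animal, play a random montage, then resume patrol at run speed.
; Patrol legs and touches share a move counter that, checked after each leg, sends it to a random side endpoint to be destroyed.
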(event `SetSize`
  (params (Value :type "Float (double-precision)"))
  (set `self.Size` Value))

(event `SetSpeed`
  (params (Value :type "Float (double-precision)"))
  (bind _output_get (set `self.Speed` Value))
  (set `CharacterMovementComponent.MaxWalkSpeed` _output_get (`self.CharacterMovement`)))

(event `UpdateMainPoint`
  (params (Location :type "Vector Structure"))
  (set `self.MainPoint` Location))

(event `MoveOutOfScreen`
  (`|AIMoveTo` self (`KismetMathLibrary.MakeVector` 2000.0) null))

(event `BoostSpeedTemporarily`
  (params (Time :type "Float (double-precision)") (Amount :type "Float (double-precision)"))
  (bind _speed (`self.Speed`))
  (set `self.OriginalSpeed` _speed)
  (set `self.Speed` (+ _speed Amount))
  (`KismetSystemLibrary.Delay` Time)
  (set `self.Speed` (`self.OriginalSpeed`)))

(event `MoveToRandomLocation`
  (params (Location :type "Vector Structure") (Radius :type "Float (double-precision)"))
  (`|AIMoveTo` self (`NavigationSystemV1.K2_GetRandomReachablePointInRadius` Location Radius null null) null))

(event `MoveToLocation`
  (params (Location :type "Vector Structure"))
  (`|AIMoveTo` self Location null))

(event `MoveToMiddle`
  (`|AIMoveTo` self (`NavigationSystemV1.K2_GetRandomReachablePointInRadius` (`self.K2_GetActorLocation` (`self.MiddlePointRef`)) 1000.0 null null) null 20.0
    (:`OnSuccess`
      (`self.StartRandomPatrol`))))

(event `StartRandomPatrol`
  ; 중앙쪽 랜덤한 위치로 순찰
  (`|AIMoveTo` self (`NavigationSystemV1.K2_GetRandomReachablePointInRadius` (`self.K2_GetActorLocation` (`self.MiddlePointRef`)) 1000.0 null null) null
    (:`OnSuccess`
      (`/Engine/EditorBlueprintResources/StandardMacros.IncrementInt` (`self.MoveCount`)
        (:`  `
          (`KismetSystemLibrary.Delay` 3.0)
          (if (>= (`self.MoveCount`) 6)
            (`self.SetSpeed` (`self.RunSpeed`))
            (`self.MoveToEndPoint`)
            (else
              (`self.SetSpeed` (`self.WalkSpeed`))
              (`self.StartRandomPatrol`))))))))

(event `ReactToTouch`
  (bind _touchmontages (`self.TouchMontages`))
  ; 터치 인터랙션
  (if (`self.IsFlyingAnimal`)
    _
    (elif (not (`self.IsReacting`))
      (`MovementComponent.StopMovementImmediately` (`self.CharacterMovement`))
      (set `self.IsReacting` true)
      (`/Engine/EditorBlueprintResources/StandardMacros.IncrementInt` (`self.MoveCount`)
        (:`  `
          (bind _returnvalue (`self.PlayAnimalMontage` (`|GetArrayItem` _touchmontages (`KismetMathLibrary.RandomIntegerInRange` 0 (`KismetArrayLibrary.Array_LastIndex` _touchmontages)))))
          (`KismetSystemLibrary.Delay` _returnvalue)
          (set `self.IsReacting` false)
          (`self.SetSpeed` (`self.RunSpeed`))
          (`self.StartRandomPatrol`))))))

(event `MoveToEndPoint`
  ; 왼쪽 혹은 오른쪽으로 이동
  (`self.SetSpeed` 150.0)
  (`|AIMoveTo` self (`self.K2_GetActorLocation` (select `bool` (`KismetMathLibrary.RandomBool`) :`false` (`self.EndPointRight`) :`true` (`self.EndPointLeft`) :!type "Actor Object Reference")) null 100.0
    (:`OnSuccess`
      (`self.K2_DestroyActor`))))

(event `self.ReceiveActorOnClicked`
  (params (ButtonPressed :type "Key Structure"))
  ; 상호작용 노드
  (`self.ReactToTouch` :!label _label))

(event `self.TouchCollision.OnComponentBeginOverlap`
  (params (OverlappedComponent :type "PrimitiveComponent Object Reference") (OtherActor :type "Actor Object Reference") (OtherComp :type "PrimitiveComponent Object Reference") (OtherBodyIndex :type Integer) (bFromSweep :type Boolean) (SweepResult :type "HitResult Structure (by ref)"))
  (if (`self.ActorHasTag` OtherActor "HandTouch")
    (`KismetSystemLibrary.PrintString` "PARENT OVERLAP")
    (`KismetSystemLibrary.Delay` 0.5)
    (`self.ReactToTouch`)))

(event `/Game/GitAssets/CJW/Interface/TouchInteract.TouchedAction`
  ; 상호작용 노드
  (goto _label))

(event `self.ReceiveBeginPlay`
  ; TargetPoint 정보 가져오기
  (bind _outactors (`GameplayStatics.GetAllActorsOfClass` "/Script/Engine.TargetPoint"))
  (for _array_element _outactors
    (if (`self.ActorHasTag` _array_element "MiddlePoint")
      (set `self.MiddlePointRef` _array_element)
      (elif (`self.ActorHasTag` _array_element "EndPointLeft")
        (set `self.EndPointLeft` _array_element)
        (elif (`self.ActorHasTag` _array_element "EndPointRight")
          (set `self.EndPointRight` _array_element)
          (elif (`self.ActorHasTag` _array_element "FixedLocation")
            (`KismetArrayLibrary.Array_Add` (`self.FixedLocation`) _array_element)
            (else
              (`KismetArrayLibrary.Array_Add` (`self.CrowLandPoints`) _array_element))))))))

(event `self.ReceiveTick`
  (params (DeltaSeconds :type "Float (single-precision)")))

(fn `PlayAnimalMontage`
  (params (Montage :type "AnimMontage Object Reference"))
  (returns (ReturnValue :type "Float (single-precision)"))
  (bind _returnvalue (`self.PlayAnimMontage` Montage))
  (return _returnvalue))

(fn `SetAnimalSpeed`
  (params (Walk :type "Float (double-precision)") (Run :type "Float (double-precision)"))
  (set `self.WalkSpeed` Walk)
  (bind _output_get (set `self.RunSpeed` Run))
  (`self.SetSpeed` _output_get))

(fn `SetIdleMontage`
  (params (IdleMontages :type "Array of AnimMontage Object Reference"))
  (set `self.IdleMontages` IdleMontages))

(fn `SetInteractMontage`
  (params (TouchMontages :type "Array of AnimMontage Object Reference"))
  (set `self.TouchMontages` TouchMontages))

(fn `UserConstructionScript`)