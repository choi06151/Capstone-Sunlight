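; Test deer doe animal Blueprint that, on BeginPlay, sets walk/run speeds and interaction montages, then starts random patrol through functions defined outside this graph.
; Local events also define random AI wandering around a middle point, moving to an end point after a move count, and a velocity-gated footstep loop with no sound assigned.
; BeginPlay calls neither event directly, and reaction, alert/run sound and main-point return logic is left disconnected.
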(event `self.ReceiveBeginPlay`
  (`parent.ReceiveBeginPlay`)
  (`self.SetAnimalSpeed` 60.0 140.0)
  (`self.SetInteractMontage` (`|MakeArray` "/Game/GitAssets/JSY/AnimalTest/Montages/DeerDoe/ANIM_GetHit_Death_Montage.ANIM_GetHit_Death_Montage" "/Game/GitAssets/JSY/AnimalTest/Montages/DeerDoe/ANIM_DeerDoe_IdleLookAround_Montage.ANIM_DeerDoe_IdleLookAround_Montage" "/Game/GitAssets/JSY/AnimalTest/Montages/DeerDoe/ANIM_DeerDoe_DownAndUP_Montage.ANIM_DeerDoe_DownAndUP_Montage" :!type "AnimMontage Object Reference"))
  (`self.StartRandomPatrol`))

(event `DeerDoeMoveRandom`
  (`|AIMoveTo` self (`NavigationSystemV1.K2_GetRandomReachablePointInRadius` (`self.K2_GetActorLocation` (`self.MiddlePointRef`)) 1000.0 null null) null 50.0
    (:`OnSuccess`
      (bind _result (`/Engine/EditorBlueprintResources/StandardMacros.IncrementInt` (`self.DeerDoeMoveCount`))
        (:`  `
          (`KismetSystemLibrary.PrintString` (`KismetStringLibrary.Conv_IntToString` _result))
          (if (>= (`self.DeerDoeMoveCount`) (`self.DeerDoeReturnEvery`))
            (`self.MoveToEndPoint`)
            (else
              (`KismetSystemLibrary.Delay` 2.0)
              (`self.DeerDoeMoveRandom`))))))))

(event `DeerDoe_Walk_Loop`
  ; 걸을 때 소리
  (`KismetSystemLibrary.Delay` 0.6)
  (if (and (> (`KismetMathLibrary.VSize` (`self.GetVelocity`)) 10.0) (not (`self.IsDeerDoeReacting`)))
    (`GameplayStatics.SpawnSoundAttached` null (`self.Mesh`) "None" (0.0 0.0 0.0) (struct) "KeepRelativeOffset" false 1.0 1.0 0.0 null null)
    (`self.DeerDoe_Walk_Loop`)
    (else
      (`self.DeerDoe_Walk_Loop`))))

(fn `UserConstructionScript`
  (`parent.UserConstructionScript`))