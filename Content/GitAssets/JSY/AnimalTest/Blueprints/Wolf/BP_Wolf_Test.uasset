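; Test wolf animal Blueprint that configures movement, interaction animations and patrol behavior on spawn.
; On BeginPlay it calls the parent, sets walk and run speeds, registers bite, howl and jump-bite montages for interaction, then starts random patrol.
; The Blueprint only supplies wolf-specific setup and defines no movement or interaction logic itself.
; Overlap and Tick events are disabled placeholders, and the construction script only calls its parent.
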(event `self.ReceiveBeginPlay`
  (`parent.ReceiveBeginPlay`)
  (`self.SetAnimalSpeed` 75.0 150.0)
  (`self.SetInteractMontage` (`|MakeArray` "/Game/GitAssets/JSY/AnimalTest/Montages/Wolf/ANIM_Wolf_Bite_Montage.ANIM_Wolf_Bite_Montage" "/Game/GitAssets/JSY/AnimalTest/Montages/Wolf/ANIM_Wolf_Howl_Montage_Montage.ANIM_Wolf_Howl_Montage_Montage" "/Game/GitAssets/JSY/AnimalTest/Montages/Wolf/ANIM_Wolf_JumpBite_Montage.ANIM_Wolf_JumpBite_Montage" :!type "AnimMontage Object Reference"))
  (`self.StartRandomPatrol`))

(fn `UserConstructionScript`
  (`parent.UserConstructionScript`))