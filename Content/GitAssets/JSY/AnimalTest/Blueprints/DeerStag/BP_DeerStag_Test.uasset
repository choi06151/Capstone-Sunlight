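; BP_DeerStag_Test is a test deer stag animal built on parent-class behavior.
; BeginPlay sets walk and run speeds and interact montages, then starts the parent's random patrol.
; Its own events define wandering around DeerStagMainPoint with a move count that triggers MoveToEndPoint, plus a delayed loop for movement sounds while not reacting.
; Alert-sprint and return-to-point logic remains in the graph but is disconnected.
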(event `self.ReceiveBeginPlay`
  (`parent.ReceiveBeginPlay`)
  (`self.SetAnimalSpeed` 60.0 140.0)
  (`self.SetInteractMontage` (`|MakeArray` "/Game/GitAssets/JSY/AnimalTest/Montages/DeerStag/ANIM_DeerStag_GetHit_Montage.ANIM_DeerStag_GetHit_Montage" "/Game/GitAssets/JSY/AnimalTest/Montages/DeerStag/ANIM_DeerStag_IdleLookAround_Montage.ANIM_DeerStag_IdleLookAround_Montage" "/Game/GitAssets/JSY/AnimalTest/Montages/DeerStag/ANIM_DeerStag_Rest_Montage.ANIM_DeerStag_Rest_Montage" :!type "AnimMontage Object Reference"))
  (`self.StartRandomPatrol`))

(event `DeerStagMoveRandom`
  (`|AIMoveTo` self (`NavigationSystemV1.K2_GetRandomReachablePointInRadius` (`self.K2_GetActorLocation` (`self.DeerStagMainPoint`)) 600.0 null null) null
    (:`OnSuccess`
      (`/Engine/EditorBlueprintResources/StandardMacros.IncrementInt` (`self.DeerStagMoveCount`)
        (:`  `
          (if (>= (`self.DeerStagMoveCount`) (`self.DeerStagReturnEvery`))
            (`self.MoveToEndPoint`)
            (else
              (`KismetSystemLibrary.Delay` 2.0)
              (`self.DeerStagMoveRandom`))))))))

(event `Deerstag_Walk_Loop`
  (`KismetSystemLibrary.Delay` 0.6)
  (if (and (> (`KismetMathLibrary.VSize` (`self.GetVelocity`)) 10.0) (not (`self.IsDeerStagReacting`)))
    (`GameplayStatics.SpawnSoundAttached` null (`self.Mesh`) "None" (0.0 0.0 0.0) (struct) "KeepRelativeOffset" false 1.0 1.0 0.0 null null)
    (`self.Deerstag_Walk_Loop`)
    (else
      (`self.Deerstag_Walk_Loop`))))

(fn `UserConstructionScript`
  (`parent.UserConstructionScript`))