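; Test bear animal Blueprint that, on BeginPlay, gives its parent class walk/run speeds and interaction montages, then starts random patrol.
; It also defines its own AIMoveTo loop that wanders around BearMainPoint, pauses between moves and periodically returns there.
; A separate delayed loop plays walk sounds while the bear moves.
; Nothing live here starts the wander loop, and the growl-and-touch-reaction chain is disconnected.
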(event `self.ReceiveBeginPlay`
  (`parent.ReceiveBeginPlay`)
  (`self.SetAnimalSpeed` 40.0 80.0)
  (`self.SetInteractMontage` (`|MakeArray` "/Game/GitAssets/JSY/AnimalTest/Montages/Bear/ANIM_Bear_Bite_Montage.ANIM_Bear_Bite_Montage" "/Game/GitAssets/JSY/AnimalTest/Montages/Bear/ANIM_Bear_GetHit4Legs_Montage.ANIM_Bear_GetHit4Legs_Montage" "/Game/GitAssets/JSY/AnimalTest/Montages/Bear/ANIM_Bear_LeftClawsAttack4LegsForward_Montage.ANIM_Bear_LeftClawsAttack4LegsForward_Montage" "/Game/GitAssets/JSY/AnimalTest/Montages/Bear/ANIM_Bear_Roar2Legs_Montage.ANIM_Bear_Roar2Legs_Montage" "/Game/GitAssets/JSY/AnimalTest/Montages/Bear/ANIM_Bear_Roar4Legs_Montage.ANIM_Bear_Roar4Legs_Montage" :!type "AnimMontage Object Reference"))
  (`self.StartRandomPatrol`))

(event `BearMoveRandom`
  (`|AIMoveTo` self (`NavigationSystemV1.K2_GetRandomReachablePointInRadius` (`self.K2_GetActorLocation` (`self.BearMainPoint`)) 300.0 null null) null 80.0
    (:`then`
      (`/Engine/EditorBlueprintResources/StandardMacros.IncrementInt` (`self.BearMoveCount`)
        (:`  `
          (if (>= (`self.BearMoveCount`) (`self.BearReturnEvery`))
            (`|AIMoveTo` self (`self.K2_GetActorLocation` (`self.BearMainPoint`)) null 80.0
              (:`OnSuccess`
                (`KismetSystemLibrary.Delay` 4.0)
                (set `self.BearMoveCount` 0)
                (`self.BearMoveRandom`)))
            (else
              (`KismetSystemLibrary.Delay` 4.0)
              (`self.BearMoveRandom`))))))))

(event `Bear_Walk_Loop`
  (`KismetSystemLibrary.Delay` 1.2)
  (if (> (`KismetMathLibrary.VSize` (`self.GetVelocity`)) 10.0)
    (`GameplayStatics.SpawnSoundAttached` "/Game/GitAssets/JSY/AnimalTest/sounds/Bear/SC_Bear_Walk_02.SC_Bear_Walk_02" null "None" (0.0 0.0 0.0) (struct) "KeepRelativeOffset" false 1.0 1.0 0.0 null null)
    (`self.Bear_Walk_Loop`)
    (else
      (`/Engine/EditorBlueprintResources/StandardMacros.IsValid` null))))

(fn `UserConstructionScript`
  (`parent.UserConstructionScript`))