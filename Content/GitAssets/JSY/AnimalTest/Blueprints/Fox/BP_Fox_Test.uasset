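; Test fox animal on a parent class, which sets walk/run speeds and interaction montages, then starts the parent's random patrol on BeginPlay.
; Its own recursive AIMoveTo wander around a main point alternates running with look-around pauses, then exits to a random endpoint and self-destroys after enough moves.
; That wander is not started from BeginPlay here, and the touch-reaction chain is disconnected.
; A separate velocity-checked loop handles walk audio.
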(event `MoveToEnd`
  (`self.SetSpeed` 250.0)
  (`|AIMoveTo` self (`self.K2_GetActorLocation` (select `bool` (`KismetMathLibrary.RandomBool`) :`false` (`self.EndPointRight`) :`true` (`self.EndPointLeft`) :!type "Actor Object Reference")) null
    (:`OnSuccess`
      (`KismetSystemLibrary.PrintString` "FOX RETURNED MAINPOINT")
      (`self.K2_DestroyActor`))))

(event `self.ReceiveBeginPlay`
  (`parent.ReceiveBeginPlay`)
  (`self.SetAnimalSpeed` 75.0 150.0)
  (`self.SetInteractMontage` (`|MakeArray` "/Game/GitAssets/JSY/AnimalTest/Montages/Fox/ANIM_Fox_Bite_Montage.ANIM_Fox_Bite_Montage" "/Game/GitAssets/JSY/AnimalTest/Montages/Fox/ANIM_Fox_GetHit_Montage.ANIM_Fox_GetHit_Montage" "/Game/GitAssets/JSY/AnimalTest/Montages/Fox/ANIM_Fox_JumpBite_Montage.ANIM_Fox_JumpBite_Montage" "/Game/GitAssets/JSY/AnimalTest/Montages/Fox/ANIM_Fox_Aggresssive_Montage.ANIM_Fox_Aggresssive_Montage" :!type "AnimMontage Object Reference"))
  (`self.StartRandomPatrol`))

(event `FoxMoveRandom`
  (`KismetSystemLibrary.Delay` (`KismetMathLibrary.RandomFloatInRange` 0.0 3.0))
  (`|AIMoveTo` self (`NavigationSystemV1.K2_GetRandomReachablePointInRadius` (`self.K2_GetActorLocation` (`self.FoxMainPoint`)) 1000.0 null null) null 40.0
    (:`OnSuccess`
      (`/Engine/EditorBlueprintResources/StandardMacros.IncrementInt` (`self.FoxMoveCount`)
        (:`  `
          (if (>= (`self.FoxMoveCount`) (`self.FoxReturnEvery`))
            (`self.MoveToEnd`)
            (else
              ; 달리거나 걷거나
              (if (== (`KismetMathLibrary.RandomIntegerInRange` 0 1) 1)
                (`KismetSystemLibrary.PrintString` "FOX RUN")
                (`self.SetSpeed` 250.0)
                (`self.FoxMoveRandom`)
                (else
                  (`SkeletalMeshComponent.PlayAnimation` (`self.Mesh`) "/Game/DriveAssets/ForestAnimalsPack/Fox/Animations/ANIM_Fox_IdleLookAround.ANIM_Fox_IdleLookAround" false)
                  (`KismetSystemLibrary.Delay` (`self.FoxPauseDelay`))
                  (`SkeletalMeshComponent.SetAnimationMode` (`self.Mesh`) "AnimationBlueprint" true)
                  (`self.SetSpeed` 80.0)
                  (`self.FoxMoveRandom`))))))))))

(event `Fox_Walk_Loop`
  (bind _foxwalkaudio (`self.FoxWalkAudio`))
  ; 소리용
  (`KismetSystemLibrary.Delay` 1.2)
  (if (> (`KismetMathLibrary.VSize` (`self.GetVelocity`)) 10.0)
    (bind _returnvalue (`GameplayStatics.SpawnSoundAttached` "/Game/GitAssets/JSY/AnimalTest/sounds/Fox/SC_Fox_Walk_01.SC_Fox_Walk_01" (`self.Mesh`) "None" (0.0 0.0 0.0) (struct) "KeepRelativeOffset" false 1.0 1.0 0.0 null null))
    (set `self.FoxWalkAudio` _returnvalue)
    (`self.Fox_Walk_Loop`)
    (else
      (`/Engine/EditorBlueprintResources/StandardMacros.IsValid` _foxwalkaudio
        (:`Is Valid`
          (`AudioComponent.Stop` _foxwalkaudio)
          (`self.Fox_Walk_Loop`))
        (:`Is Not Valid`
          (`self.Fox_Walk_Loop`))))))

(fn `UserConstructionScript`
  (`parent.UserConstructionScript`))