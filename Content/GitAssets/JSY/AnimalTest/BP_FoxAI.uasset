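; BP_FoxAI is a test fox character that wanders on its own and periodically plays a bite animation.
; A looping idle-and-move cycle waits, then sends the pawn to a random reachable navmesh point within a radius, restarting whether the move succeeds or fails.
; A separate looping timer plays the bite montage at fixed intervals, independent of movement and without any targeting or damage logic.
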(event `self.ReceiveBeginPlay`
  (`KismetSystemLibrary.K2_SetTimerDelegate` (delegate `BiteAttack`) 10.0 true)
  (`self.StartIdle`))

(event `BiteAttack`
  (`self.PlayAnimMontage` "/Game/GitAssets/JSY/AnimalTest/ANIM_Fox_Bite_Montage.ANIM_Fox_Bite_Montage"))

(event `StartIdle`
  (`KismetSystemLibrary.Delay` (`self.WaitTime`))
  (`self.StartMoveRandom`))

(event `StartMoveRandom`
  (`|AIMoveTo` self (`NavigationSystemV1.K2_GetRandomReachablePointInRadius` (`self.K2_GetActorLocation`) (`self.MoveRadius`) null null) null
    (:`OnSuccess`
      (`self.StartIdle`))
    (:`OnFail`
      (`self.StartIdle`))))

(fn `UserConstructionScript`)