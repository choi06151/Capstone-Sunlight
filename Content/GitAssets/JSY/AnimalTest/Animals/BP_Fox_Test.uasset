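; BP_Fox_Test is a test Blueprint for a fox animal that patrols randomly and reacts to touch.
; On BeginPlay it runs the parent logic, prints debug messages and calls StartRandomPatrol.
; A TouchCollision overlap calls ReactToTouch after a half-second delay, for any overlapping actor because the HandTouch tag check is disconnected.
; Neither StartRandomPatrol nor ReactToTouch is defined in this Blueprint.
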(event `self.ReceiveBeginPlay`
  (`parent.ReceiveBeginPlay`)
  (`KismetSystemLibrary.PrintString` "FOX BEGIN")
  (`KismetSystemLibrary.PrintString` "BEFORE PATROL")
  (`self.StartRandomPatrol`))

(event `self.TouchCollision.OnComponentBeginOverlap`
  (params (OverlappedComponent :type "PrimitiveComponent Object Reference") (OtherActor :type "Actor Object Reference") (OtherComp :type "PrimitiveComponent Object Reference") (OtherBodyIndex :type Integer) (bFromSweep :type Boolean) (SweepResult :type "HitResult Structure (by ref)"))
  (`KismetSystemLibrary.Delay` 0.5)
  (`self.ReactToTouch`))

(fn `UserConstructionScript`
  (`parent.UserConstructionScript`))