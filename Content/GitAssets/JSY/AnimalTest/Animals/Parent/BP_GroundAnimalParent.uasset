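; BP_GroundAnimalParent is a parent Character for ground animals, exposing movement, montage and setter events.
; AI MoveTo drives travel to a given, random reachable or fixed exit point, and a random patrol that repeats after a delay on success or failure.
; ReactToTouch plays the touch montage; BeginPlay is empty.
; SetSpeed updates max walk speed, while the temporary boost changes only the Speed variable and SetSize only stores its value.
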(event `MoveToLocation`
  (params (Location :type "Vector Structure"))
  (`|AIMoveTo` self Location null))

(event `MoveToRandomLocation`
  (params (Location :type "Vector Structure") (Radius :type "Float (double-precision)"))
  (`|AIMoveTo` self (`NavigationSystemV1.K2_GetRandomReachablePointInRadius` Location Radius null null) null))

(event `SetSpeed`
  (params (Value :type "Float (double-precision)"))
  (bind _output_get (set `self.Speed` Value))
  (set `CharacterMovementComponent.MaxWalkSpeed` _output_get (`self.CharacterMovement`)))

(event `SetSize`
  (params (Value :type "Float (double-precision)"))
  (set `self.Size` Value))

(event `UpdateMainPoint`
  (params (Location :type "Vector Structure"))
  (set `self.MainPoint` Location))

(event `PlayAnimalMontage`
  (params (Montage :type "AnimMontage Object Reference"))
  (`self.PlayAnimMontage` Montage))

(event `MoveOutOfScreen`
  (`|AIMoveTo` self (`KismetMathLibrary.MakeVector` 2000.0) null))

(event `StartRandomPatrol`
  (`|AIMoveTo` self (`NavigationSystemV1.K2_GetRandomReachablePointInRadius` (`self.K2_GetActorLocation`) 1000.0 null null) null
    (:`OnSuccess`
      _)
    (:`OnFail`
      _))
  (`KismetSystemLibrary.Delay` 3.0)
  (`self.StartRandomPatrol`))

(event `BoostSpeedTemporarily`
  (params (Time :type "Float (double-precision)") (Amount :type "Float (double-precision)"))
  (bind _speed (`self.Speed`))
  (set `self.OriginalSpeed` _speed)
  (set `self.Speed` (+ _speed Amount))
  (`KismetSystemLibrary.Delay` Time)
  (set `self.Speed` (`self.OriginalSpeed`)))

(event `self.ReceiveBeginPlay`)

(event `ReactToTouch`
  (`self.PlayAnimalMontage` (`self.TouchMontage`)))

(fn `UserConstructionScript`)