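; Tree actor whose species and level select its skeletal mesh and falling-particle effect, with particles enabled only if the player is nearby when set.
; Tick eases the BPA_rotate_master anim instance's rotation toward a target.
; An overlapping BP_Light stops the Wind timeline and sets a slight directional tilt; leaving starts randomized wind sway.
; SwingTree briefly boosts wind strength and speed, bursting species-specific particles at level 5 and above.
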(event `SetTree`
  (params (Input :type "/Game/GitAssets/CJW/Enum/E_TreeType Enum" :default "NewEnumerator0") (Level :type Integer))
  (set `self.Treetype` Input)
  (set `self.Leveled` Level)
  (`self.SetSkeletonMesh` Input Level)
  (`|ExecutionSequence`
    (:`then_0`
      (`self.SetNiagara` true Input Level))
    (:`then_1`
      (switch `/Game/GitAssets/CJW/Enum/E_TreeType` Input))))

(event `self.ReceiveBeginPlay`)

(event `self.ReceiveTick`
  (params (DeltaSeconds :type "Float (single-precision)"))
  (bind _as_bpa_rotate_master (`self.As BPA Rotate Master`))
  (set `/Game/GitAssets/KDH/BP+BPA/BPA_rotate_master.rotate` (`KismetMathLibrary.RInterpTo` (`/Game/GitAssets/KDH/BP+BPA/BPA_rotate_master.rotate` _as_bpa_rotate_master) (`/Game/GitAssets/KDH/BP+BPA/BPA_rotate_master.targetrotate` _as_bpa_rotate_master) DeltaSeconds 1.0) (`self.As BPA Rotate Master`)))

(event `self.Sphere.OnComponentEndOverlap`
  (params (OverlappedComponent :type "PrimitiveComponent Object Reference") (OtherActor :type "Actor Object Reference") (OtherComp :type "PrimitiveComponent Object Reference") (OtherBodyIndex :type Integer))
  (cast `/Game/GitAssets/CJW/Blueprints/BP_Light` OtherActor)
  (bind (_direction _newtrack_0) (`Timeline|Wind` :!label _label)
    (:`Update`
      (set `/Game/GitAssets/KDH/BP+BPA/BPA_rotate_master.targetrotate` (`KismetMathLibrary.MakeRotator` (* _newtrack_0 (`KismetMathLibrary.RandomFloatInRange` 0.0 (`self.WindStrength`))) (* _newtrack_0 (`KismetMathLibrary.RandomFloatInRange` 0.0 (`self.WindStrength`)))) (`self.As BPA Rotate Master`)))))

(event `self.Sphere.OnComponentBeginOverlap`
  (params (OverlappedComponent :type "PrimitiveComponent Object Reference") (OtherActor :type "Actor Object Reference") (OtherComp :type "PrimitiveComponent Object Reference") (OtherBodyIndex :type Integer) (bFromSweep :type Boolean) (SweepResult :type "HitResult Structure (by ref)"))
  (bind _asbp_light (cast `/Game/GitAssets/CJW/Blueprints/BP_Light` OtherActor))
  (bind (_returnvalue_x _returnvalue_y) (`KismetMathLibrary.BreakVector` (`KismetMathLibrary.InverseTransformDirection` (`self.GetTransform`) (`KismetMathLibrary.Normal` (- (`self.K2_GetActorLocation` _asbp_light) (`self.K2_GetActorLocation`))))))
  (set `/Game/GitAssets/KDH/BP+BPA/BPA_rotate_master.targetrotate` (`KismetMathLibrary.MakeRotator` (* 3.0 _returnvalue_y) (* _returnvalue_x -3.0)) (`self.As BPA Rotate Master`))
  (goto _label :!via `Stop`))

(event `SwingTree`
  (set `self.WindStrength` 5.0)
  (`TimelineComponent.SetPlayRate` (`self.Wind`) 5.0)
  (`|ExecutionSequence`
    (:`then_0`
      (`KismetSystemLibrary.Delay` 2.0 :!label _label_2)
      (set `self.WindStrength` 0.3)
      (`TimelineComponent.SetPlayRate` (`self.Wind`) 1.0))
    (:`then_1`
      (if (>= (`self.Leveled`) 5)
        (`NiagaraFunctionLibrary.SpawnSystemAtLocation` (select `/Game/GitAssets/CJW/Enum/E_TreeType` (`self.TreeType`) :`NewEnumerator0` "/Game/GitAssets/CJW/VFX/Busrt/NS_BurstFallingBlossom.NS_BurstFallingBlossom" :`NewEnumerator1` "/Game/GitAssets/CJW/VFX/Falling/NS_FallingLeaves_Maple.NS_FallingLeaves_Maple" :`NewEnumerator2` "/Game/GitAssets/CJW/VFX/Falling/NS_FallingLeaves_GreenLeaf.NS_FallingLeaves_GreenLeaf" :`NewEnumerator3` "/Game/GitAssets/CJW/VFX/Busrt/NS_BurstFallingSnow.NS_BurstFallingSnow" :`NewEnumerator4` "/Game/GitAssets/CJW/VFX/Busrt/NS_BurstFallingBlossom.NS_BurstFallingBlossom" :!type "NiagaraSystem Object Reference") (+ (`SceneComponent.K2_GetComponentLocation` (`self.Niagara`)) (0.0 0.0 50.0)))
        (goto _label_2)))))

(fn `SetNiagara`
  (params (Active :type Boolean) (Index :type "/Game/GitAssets/CJW/Enum/E_TreeType Enum" :default "NewEnumerator0") (Index1 :type Integer))
  (if Active
    (if (<= (`KismetMathLibrary.Vector_Distance` (`self.K2_GetActorLocation` (`GameplayStatics.GetPlayerCharacter` 0)) (`self.K2_GetActorLocation`)) 5000.0)
      (`NiagaraComponent.SetAsset` (`self.Niagara`) (select `/Game/GitAssets/CJW/Enum/E_TreeType` Index :`NewEnumerator0` "/Game/GitAssets/CJW/VFX/Falling/NS_CherryBlossomSystem.NS_CherryBlossomSystem" :`NewEnumerator1` "/Game/GitAssets/CJW/VFX/Falling/NS_FallingLeaves_Maple.NS_FallingLeaves_Maple" :`NewEnumerator2` "/Game/GitAssets/CJW/VFX/Falling/NS_FallingLeaves_GreenLeaf.NS_FallingLeaves_GreenLeaf" :!type "NiagaraSystem Object Reference") false)
      (`NiagaraComponent.SetVariableFloat` (`self.Niagara`) "SpawnRate" (select `int` Index1 :`0` 0.0 :`1` 5.0 :`2` 10.0 :`3` 15.0 :`4` 20.0 :`5` 25.0 :`6` 30.0 :`7` 35.0 :`8` 40.0 :`9` 30.0 :`10` 25.0 :`11` 20.0 :`12` 15.0 :`13` 10.0 :`14` 8.0 :`15` 5.0 :`16` 3.0 :`17` 1.0 :`18` 0.0 :!type "Float (single-precision)"))
      (switch `/Game/GitAssets/CJW/Enum/E_TreeType` Index
        (:`NewEnumerator1`
          (`NiagaraComponent.SetVariableLinearColor` (`self.Niagara`) "Color" (select `int` Index1 :`0` (struct :`R` 0.133 :`G` 0.545 :`B` 0.133 :`A` 1.0) :`1` (struct :`R` 0.196 :`G` 0.627 :`B` 0.196 :`A` 1.0) :`2` (struct :`R` 0.333 :`G` 0.667 :`B` 0.235 :`A` 1.0) :`3` (struct :`R` 0.471 :`G` 0.706 :`B` 0.196 :`A` 1.0) :`4` (struct :`R` 0.627 :`G` 0.745 :`B` 0.157 :`A` 1.0) :`5` (struct :`R` 0.784 :`G` 0.784 :`B` 0.118 :`A` 1.0) :`6` (struct :`R` 0.863 :`G` 0.627 :`B` 0.157 :`A` 1.0) :`7` (struct :`R` 0.863 :`G` 0.431 :`B` 0.118 :`A` 1.0) :`8` (struct :`R` 0.784 :`G` 0.314 :`B` 0.157 :`A` 1.0) :`9` (struct :`R` 0.745 :`G` 0.353 :`B` 0.196 :`A` 1.0) :`10` (struct :`R` 0.667 :`G` 0.392 :`B` 0.235 :`A` 1.0) :`11` (struct :`R` 0.864583 :`G` 0.392 :`B` 0.275 :`A` 1.0) :`12` (struct :`R` 0.549 :`G` 0.353 :`B` 0.235 :`A` 1.0) :`13` (struct :`R` 0.51 :`G` 0.314 :`B` 0.196 :`A` 1.0) :`14` (struct :`R` 0.431 :`G` 0.275 :`B` 0.157 :`A` 1.0) :`15` (struct :`R` 1.0 :`G` 0.255 :`B` 0.137 :`A` 1.0) :`16` (struct :`R` 0.392 :`G` 0.235 :`B` 0.118 :`A` 1.0) :`17` (struct :`R` 0.275 :`G` 0.196 :`B` 0.098 :`A` 1.0) :`18` (struct :`R` 0.275 :`G` 0.196 :`B` 0.098 :`A` 1.0) :!type "LinearColor Structure"))))
      (else
        (`NiagaraComponent.SetAsset` (`self.Niagara`) null true)))
    (else
      (`NiagaraComponent.SetAsset` (`self.Niagara`) null true))))

(fn `SetSkeletonMesh`
  (params (Input :type "/Game/GitAssets/CJW/Enum/E_TreeType Enum" :default "NewEnumerator0") (Level :type Integer))
  (bind _leveled (`self.Leveled`))
  (`SkeletalMeshComponent.SetSkeletalMeshAsset` (`self.SkeletalMesh`) (select `/Game/GitAssets/CJW/Enum/E_TreeType` Input :`NewEnumerator0` (select `int` _leveled :`0` "/Game/DriveAssets/ForShare/CJW/Tree/CherryBlossom/Type1/CherryTree1.CherryTree1" :`1` "/Game/DriveAssets/ForShare/CJW/Tree/CherryBlossom/Type1/CherryTree2.CherryTree2" :`2` "/Game/DriveAssets/ForShare/CJW/Tree/CherryBlossom/Type1/CherryTree3.CherryTree3" :`3` "/Game/DriveAssets/ForShare/CJW/Tree/CherryBlossom/Type1/CherryTree4.CherryTree4" :`4` "/Game/DriveAssets/ForShare/CJW/Tree/CherryBlossom/Type1/CherryTree5.CherryTree5" :`5` "/Game/DriveAssets/ForShare/CJW/Tree/CherryBlossom/Type1/CherryTree6.CherryTree6" :`6` "/Game/DriveAssets/ForShare/CJW/Tree/CherryBlossom/Type1/CherryTree7.CherryTree7" :`7` "/Game/DriveAssets/ForShare/CJW/Tree/CherryBlossom/Type1/CherryTree8.CherryTree8" :`8` "/Game/DriveAssets/ForShare/CJW/Tree/CherryBlossom/Type1/CherryTree9.CherryTree9" :`9` "/Game/DriveAssets/ForShare/CJW/Tree/CherryBlossom/Type1/CherryTree10.CherryTree10" :`10` "/Game/DriveAssets/ForShare/CJW/Tree/CherryBlossom/Type1/CherryTree9.CherryTree9" :`11` "/Game/DriveAssets/ForShare/CJW/Tree/CherryBlossom/Type1/CherryTree8.CherryTree8" :`12` "/Game/DriveAssets/ForShare/CJW/Tree/CherryBlossom/Type1/CherryTree7.CherryTree7" :`13` "/Game/DriveAssets/ForShare/CJW/Tree/CherryBlossom/Type1/CherryTree6.CherryTree6" :`14` "/Game/DriveAssets/ForShare/CJW/Tree/CherryBlossom/Type1/CherryTree5.CherryTree5" :`15` "/Game/DriveAssets/ForShare/CJW/Tree/CherryBlossom/Type1/CherryTree4.CherryTree4" :`16` "/Game/DriveAssets/ForShare/CJW/Tree/CherryBlossom/Type1/CherryTree17.CherryTree17" :`17` "/Game/DriveAssets/ForShare/CJW/Tree/CherryBlossom/Type1/CherryTree18.CherryTree18" :`18` "/Game/DriveAssets/ForShare/CJW/Tree/CherryBlossom/Type1/CherryTree19.CherryTree19" :!type "SkeletalMesh Object Reference") :`NewEnumerator1` (select `int` _leveled :`0` "/Game/DriveAssets/ForShare/CJW/Tree/Maple/Type1/MapleTree2.MapleTree2" :`1` "/Game/DriveAssets/ForShare/CJW/Tree/Maple/Type1/MapleTree2.MapleTree2" :`2` "/Game/DriveAssets/ForShare/CJW/Tree/Maple/Type1/MapleTree3.MapleTree3" :`3` "/Game/DriveAssets/ForShare/CJW/Tree/Maple/Type1/MapleTree4.MapleTree4" :`4` "/Game/DriveAssets/ForShare/CJW/Tree/Maple/Type1/MapleTree5.MapleTree5" :`5` "/Game/DriveAssets/ForShare/CJW/Tree/Maple/Type1/MapleTree6.MapleTree6" :`6` "/Game/DriveAssets/ForShare/CJW/Tree/Maple/Type1/MapleTree7.MapleTree7" :`7` "/Game/DriveAssets/ForShare/CJW/Tree/Maple/Type1/MapleTree8.MapleTree8" :`8` "/Game/DriveAssets/ForShare/CJW/Tree/Maple/Type1/MapleTree9.MapleTree9" :`9` "/Game/DriveAssets/ForShare/CJW/Tree/Maple/Type1/MapleTree10.MapleTree10" :`10` "/Game/DriveAssets/ForShare/CJW/Tree/Maple/Type1/MapleTree9.MapleTree9" :`11` "/Game/DriveAssets/ForShare/CJW/Tree/Maple/Type1/MapleTree8.MapleTree8" :`12` "/Game/DriveAssets/ForShare/CJW/Tree/Maple/Type1/MapleTree7.MapleTree7" :`13` "/Game/DriveAssets/ForShare/CJW/Tree/Maple/Type1/MapleTree6.MapleTree6" :`14` "/Game/DriveAssets/ForShare/CJW/Tree/Maple/Type1/MapleTree5.MapleTree5" :`15` "/Game/DriveAssets/ForShare/CJW/Tree/Maple/Type1/MapleTree4.MapleTree4" :`16` "/Game/DriveAssets/ForShare/CJW/Tree/Maple/Type1/MapleTree3.MapleTree3" :`17` "/Game/DriveAssets/ForShare/CJW/Tree/Maple/Type1/MapleTree2.MapleTree2" :`18` "/Game/DriveAssets/ForShare/CJW/Tree/CherryBlossom/Type1/CherryTree1.CherryTree1" :!type "SkeletalMesh Object Reference") :`NewEnumerator2` (select `int` _leveled :`0` "/Game/DriveAssets/ForShare/CJW/Tree/European2/Type1/European2.European2" :`1` "/Game/DriveAssets/ForShare/CJW/Tree/European2/European2-1.European2-1" :`2` "/Game/DriveAssets/ForShare/CJW/Tree/European2/Type1/European3.European3" :`3` "/Game/DriveAssets/ForShare/CJW/Tree/European2/Type1/European4.European4" :`4` "/Game/DriveAssets/ForShare/CJW/Tree/European2/Type1/European5.European5" :`5` "/Game/DriveAssets/ForShare/CJW/Tree/European2/Type1/European6.European6" :`6` "/Game/DriveAssets/ForShare/CJW/Tree/European2/Type1/European7.European7" :`7` "/Game/DriveAssets/ForShare/CJW/Tree/European2/Type1/European8.European8" :`8` "/Game/DriveAssets/ForShare/CJW/Tree/European2/Type1/European9.European9" :`9` "/Game/DriveAssets/ForShare/CJW/Tree/European2/Type1/European10.European10" :`10` "/Game/DriveAssets/ForShare/CJW/Tree/European2/Type1/European9.European9" :`11` "/Game/DriveAssets/ForShare/CJW/Tree/European2/Type1/European8.European8" :`12` "/Game/DriveAssets/ForShare/CJW/Tree/European2/Type1/European7.European7" :`13` "/Game/DriveAssets/ForShare/CJW/Tree/European2/Type1/European6.European6" :`14` "/Game/DriveAssets/ForShare/CJW/Tree/European2/Type1/European5.European5" :`15` "/Game/DriveAssets/ForShare/CJW/Tree/European2/Type1/European4.European4" :`16` "/Game/DriveAssets/ForShare/CJW/Tree/European2/Type1/European3.European3" :`17` "/Game/DriveAssets/ForShare/CJW/Tree/European2/European16.European16" :`18` "/Game/DriveAssets/ForShare/CJW/Tree/European2/European17.European17" :!type "SkeletalMesh Object Reference") :`NewEnumerator3` "/Game/DriveAssets/ForShare/CJW/Tree/CherryBlossom/Type1/CherryTree1.CherryTree1" :`NewEnumerator4` "/Game/DriveAssets/ForShare/CJW/Tree/CherryBlossom/Type1/CherryTree1.CherryTree1"))
  (bind _asbpa_rotate_master (cast `/Game/GitAssets/KDH/BP+BPA/BPA_rotate_master` (`SkeletalMeshComponent.GetAnimInstance` (`self.SkeletalMesh`))))
  (set `self.As BPA Rotate Master` _asbpa_rotate_master))

(fn `UserConstructionScript`)

(fn `새 함수`)