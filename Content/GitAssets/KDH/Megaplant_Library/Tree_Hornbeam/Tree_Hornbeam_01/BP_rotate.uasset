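; BP_rotate is an actor, stored with the Hornbeam tree assets, that tilts its skeletal mesh in reaction to actors overlapping its capsule.
; On overlap, it projects the direction to the other actor onto its forward and right vectors, setting a small roll and yaw target on the BPA_rotate AnimInstance.
; Tick eases the AnimInstance's Rotate toward that target with RInterpTo.
; No end-overlap handler resets the target.
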(event `self.ReceiveTick`
  (params (DeltaSeconds :type "Float (single-precision)"))
  (bind _asbpa_rotate (cast `/Game/GitAssets/KDH/Megaplant_Library/Tree_Hornbeam/Tree_Hornbeam_01/BPA_rotate` (`SkeletalMeshComponent.GetAnimInstance` (`self.SkeletalMesh`))))
  (set `/Game/GitAssets/KDH/Megaplant_Library/Tree_Hornbeam/Tree_Hornbeam_01/BPA_rotate.rotate` (`KismetMathLibrary.RInterpTo` (`/Game/GitAssets/KDH/Megaplant_Library/Tree_Hornbeam/Tree_Hornbeam_01/BPA_rotate.rotate` _asbpa_rotate) (`/Game/GitAssets/KDH/Megaplant_Library/Tree_Hornbeam/Tree_Hornbeam_01/BPA_rotate.targetrotate` _asbpa_rotate) DeltaSeconds 1.0) _asbpa_rotate))

(event `self.Capsule.OnComponentBeginOverlap`
  (params (OverlappedComponent :type "PrimitiveComponent Object Reference") (OtherActor :type "Actor Object Reference") (OtherComp :type "PrimitiveComponent Object Reference") (OtherBodyIndex :type Integer) (bFromSweep :type Boolean) (SweepResult :type "HitResult Structure (by ref)"))
  (bind _returnvalue (`KismetMathLibrary.Normal` (- (`self.K2_GetActorLocation` OtherActor) (`self.K2_GetActorLocation`))))
  (bind _asbpa_rotate (cast `/Game/GitAssets/KDH/Megaplant_Library/Tree_Hornbeam/Tree_Hornbeam_01/BPA_rotate` (`SkeletalMeshComponent.GetAnimInstance` (`self.SkeletalMesh`))))
  (set `/Game/GitAssets/KDH/Megaplant_Library/Tree_Hornbeam/Tree_Hornbeam_01/BPA_rotate.targetrotate` (`KismetMathLibrary.MakeRotator` (* (`KismetMathLibrary.Dot_VectorVector` _returnvalue (`self.GetActorForwardVector`)) 3.0) 0.0 (* (`KismetMathLibrary.Dot_VectorVector` _returnvalue (`self.GetActorRightVector`)) 3.0)) _asbpa_rotate))

(fn `UserConstructionScript`)

(fn `새 함수`)